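; ArkFrame base class for item container structures that lets mods attach logic expansion objects.
; After a delayed authority-side start (or unstasis), it fetches expansion templates from the ArkFrame manager, polling until ready, and builds the expansions.
; Templates are cached on the class default object per session ID, so later instances skip the request.
; Overridden structure events call the parent, then forward to every expansion; multi-use entries get reserved indices per expansion.
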(event Custom|Delayed_GetNegotiatorData
  ;[1 1 1] On timer tick, check to see if the CDO has already been updated first
  (bind _returnvalue (Class|VictoryCore|GetClassDefaultObject (Utilities|GetClass self)))
  (bind _asarkframe_structure_itemcontainerbasebp_c (Utilities|Casting|CastToArkFrame_Structure_ItemContainerBaseBP _returnvalue)
    (:then
      (if (== (Variables|ArkFrame_Structure_ItemContainerBaseBP_C|GetCDO_Session_ID _asarkframe_structure_itemcontainerbasebp_c) (CallFunction|GetArkFrameSessionID))
        (Variables|ArkFrame|System|SetLogicExpansionTemplates (Variables|ArkFrame_Structure_ItemContainerBaseBP_C|GetLogicExpansionTemplates _asarkframe_structure_itemcontainerbasebp_c))
        (Variables|ArkFrame|System|SetCDO_Session_ID (Variables|ArkFrame_Structure_ItemContainerBaseBP_C|GetCDO_Session_ID _asarkframe_structure_itemcontainerbasebp_c))
        (CallFunction|BuildModExtensionObjects)
        (Utilities|Time|ClearTimerbyFunctionName 0 "Delayed_GetNegotiatorData" :!label _label)
        (else
          ;[1 1 1] if not, Make sure ArkFrame is ready
          (if (CallFunction|CheckArkFrameReadiness)
            ;[1 1 1] Request data from the Arkframe sytem, and set the CDO data as well
            (Utilities|Time|ClearTimerbyFunctionName 0 "Delayed_GetNegotiatorData")
            (bind _logicexpansiontemplates (Class|ArkFrameManagerInterface|GetLogicExpansions(Message) (CallFunction|GetArkFrameManager) (Variables|ArkFrame|GetUniqueName) (Variables|ArkFrame|GetDescriptiveTags)))
            (Variables|ArkFrame|System|SetLogicExpansionTemplates _logicexpansiontemplates)
            (Variables|ArkFrame|System|SetCDO_Session_ID (CallFunction|GetArkFrameSessionID))
            (Utilities|FlowControl|Sequence
              (:then_0
                (bind _returnvalue_2 (Class|VictoryCore|GetClassDefaultObject (Utilities|GetClass self)))
                (bind _asarkframe_structure_itemcontainerbasebp_c_2 (Utilities|Casting|CastToArkFrame_Structure_ItemContainerBaseBP _returnvalue_2))
                (Variables|ArkFrame_Structure_ItemContainerBaseBP_C|SetLogicExpansionTemplates _asarkframe_structure_itemcontainerbasebp_c_2 (Variables|ArkFrame|System|GetLogicExpansionTemplates))
                (Variables|ArkFrame_Structure_ItemContainerBaseBP_C|SetCDO_Session_ID _asarkframe_structure_itemcontainerbasebp_c_2 (Variables|ArkFrame|System|GetCDO_Session_ID)))
              (:then_1
                (CallFunction|BuildModExtensionObjects)))))))
    (:CastFailed
      (goto _label))))

(event Custom|BuildModExtensionObjects
  ;[1 1 1] Generate mod related sub-objects
  (Utilities|ConstructLogicExpansions (Variables|ArkFrame|System|GetLogicExpansionTemplates) (Variables|ArkFrame|System|GetLogicExpansions) self
    (:OutExec
      (Networking|ForceNetUpdate))))

(event Custom|Delayed%20EBP_ArkFrameBridge
  ;[1 1 1] Get ArkFrame Startup Conditions and proceed to instantiation if appropriate
  (if (not (Variables|Default|GetbStasised))
    (Utilities|FlowControl|DoOnce false
      (:Completed
        ;[1 1 1] Check for if this object was generated from a current CDO
        (if (== (Variables|ArkFrame|System|GetCDO_Session_ID) (CallFunction|GetArkFrameSessionID))
          (CallFunction|BuildModExtensionObjects)
          (else
            ;[1 1 1] If not then check if the CDO has already been updated for this session
            (bind _returnvalue (Class|VictoryCore|GetClassDefaultObject (Utilities|GetClass self)))
            (bind _asarkframe_structure_itemcontainerbasebp_c (Utilities|Casting|CastToArkFrame_Structure_ItemContainerBaseBP _returnvalue))
            (if (== (Variables|ArkFrame_Structure_ItemContainerBaseBP_C|GetCDO_Session_ID _asarkframe_structure_itemcontainerbasebp_c) (CallFunction|GetArkFrameSessionID))
              (Variables|ArkFrame|System|SetLogicExpansionTemplates (Variables|ArkFrame_Structure_ItemContainerBaseBP_C|GetLogicExpansionTemplates _asarkframe_structure_itemcontainerbasebp_c))
              (Variables|ArkFrame|System|SetCDO_Session_ID (Variables|ArkFrame_Structure_ItemContainerBaseBP_C|GetCDO_Session_ID _asarkframe_structure_itemcontainerbasebp_c))
              (CallFunction|BuildModExtensionObjects)
              (else
                ;[1 1 1] If not, check if the AF system is ready, otherwise set the retry timer
                (if (CallFunction|CheckArkFrameReadiness)
                  ;[1 1 1] Request data from the Arkframe sytem, and set the CDO data as well
                  (Utilities|Time|ClearTimerbyFunctionName 0 "Delayed_GetNegotiatorData")
                  (bind _logicexpansiontemplates (Class|ArkFrameManagerInterface|GetLogicExpansions(Message) (CallFunction|GetArkFrameManager) (Variables|ArkFrame|GetUniqueName) (Variables|ArkFrame|GetDescriptiveTags)))
                  (Variables|ArkFrame|System|SetLogicExpansionTemplates _logicexpansiontemplates)
                  (Variables|ArkFrame|System|SetCDO_Session_ID (CallFunction|GetArkFrameSessionID))
                  (Utilities|FlowControl|Sequence
                    (:then_0
                      (bind _returnvalue_2 (Class|VictoryCore|GetClassDefaultObject (Utilities|GetClass self)))
                      (bind _asarkframe_structure_itemcontainerbasebp_c_2 (Utilities|Casting|CastToArkFrame_Structure_ItemContainerBaseBP _returnvalue_2))
                      (Variables|ArkFrame_Structure_ItemContainerBaseBP_C|SetLogicExpansionTemplates _asarkframe_structure_itemcontainerbasebp_c_2 (Variables|ArkFrame|System|GetLogicExpansionTemplates))
                      (Variables|ArkFrame_Structure_ItemContainerBaseBP_C|SetCDO_Session_ID _asarkframe_structure_itemcontainerbasebp_c_2 (Variables|ArkFrame|System|GetCDO_Session_ID)))
                    (:then_1
                      (CallFunction|BuildModExtensionObjects)))
                  (else
                    (Utilities|Time|SetTimerbyFunctionName 0 "Delayed_GetNegotiatorData" 0.5 true)))))))))))

(event EventBeginPlay
  ;[1 1 1] Get ArkFrame Startup Conditions and proceed to instantiation if appropriate
  (|CallParentFunction)
  (Utilities|FlowControl|Delay 2.0)
  (Networking|SwitchHasAuthority
    (:Authority
      (Utilities|Time|SetTimerbyEvent (delegate Custom|Delayed%20EBP_ArkFrameBridge) 1e+01))))

(event EventBPUnstasis
  ;[1 1 1] Get ArkFrame Startup Conditions and proceed to instantiation if appropriate
  (|CallParentFunction)
  (Utilities|FlowControl|Sequence
    (:then_0
      (Networking|SwitchHasAuthority
        (:Authority
          (Utilities|FlowControl|Delay 2.0)
          (Utilities|FlowControl|DoOnce false
            (:Completed
              ;[1 1 1] Check for if this object was generated from a current CDO
              (if (== (Variables|ArkFrame|System|GetCDO_Session_ID) (CallFunction|GetArkFrameSessionID))
                (CallFunction|BuildModExtensionObjects)
                (else
                  ;[1 1 1] If not then check if the CDO has already been updated for this session
                  (bind _returnvalue (Class|VictoryCore|GetClassDefaultObject (Utilities|GetClass self)))
                  (bind _asarkframe_structure_itemcontainerbasebp_c (Utilities|Casting|CastToArkFrame_Structure_ItemContainerBaseBP _returnvalue))
                  (if (== (Variables|ArkFrame_Structure_ItemContainerBaseBP_C|GetCDO_Session_ID _asarkframe_structure_itemcontainerbasebp_c) (CallFunction|GetArkFrameSessionID))
                    (Variables|ArkFrame|System|SetLogicExpansionTemplates (Variables|ArkFrame_Structure_ItemContainerBaseBP_C|GetLogicExpansionTemplates _asarkframe_structure_itemcontainerbasebp_c))
                    (Variables|ArkFrame|System|SetCDO_Session_ID (Variables|ArkFrame_Structure_ItemContainerBaseBP_C|GetCDO_Session_ID _asarkframe_structure_itemcontainerbasebp_c))
                    (CallFunction|BuildModExtensionObjects)
                    (else
                      ;[1 1 1] If not, check if the AF system is ready, otherwise set the retry timer
                      (if (CallFunction|CheckArkFrameReadiness)
                        ;[1 1 1] Request data from the Arkframe sytem, and set the CDO data as well
                        (Utilities|Time|ClearTimerbyFunctionName 0 "Delayed_GetNegotiatorData")
                        (bind _logicexpansiontemplates (Class|ArkFrameManagerInterface|GetLogicExpansions(Message) (CallFunction|GetArkFrameManager) (Variables|ArkFrame|GetUniqueName) (Variables|ArkFrame|GetDescriptiveTags)))
                        (Variables|ArkFrame|System|SetLogicExpansionTemplates _logicexpansiontemplates)
                        (Variables|ArkFrame|System|SetCDO_Session_ID (CallFunction|GetArkFrameSessionID))
                        (Utilities|FlowControl|Sequence
                          (:then_0
                            (bind _returnvalue_2 (Class|VictoryCore|GetClassDefaultObject (Utilities|GetClass self)))
                            (bind _asarkframe_structure_itemcontainerbasebp_c_2 (Utilities|Casting|CastToArkFrame_Structure_ItemContainerBaseBP _returnvalue_2))
                            (Variables|ArkFrame_Structure_ItemContainerBaseBP_C|SetLogicExpansionTemplates _asarkframe_structure_itemcontainerbasebp_c_2 (Variables|ArkFrame|System|GetLogicExpansionTemplates))
                            (Variables|ArkFrame_Structure_ItemContainerBaseBP_C|SetCDO_Session_ID _asarkframe_structure_itemcontainerbasebp_c_2 (Variables|ArkFrame|System|GetCDO_Session_ID)))
                          (:then_1
                            (CallFunction|BuildModExtensionObjects)))
                        (else
                          (Utilities|Time|SetTimerbyFunctionName 0 "Delayed_GetNegotiatorData" 0.5 true))))))))))))
    (:then_1
      (Class|ArkFrameLogicExpansionInterface|ExpandedBPUnstasis(Message) (Variables|ArkFrame|System|GetLogicExpansions)))))

(fn ConstructionScript
  (|CallParentFunction))

(fn PowerGeneratorBuiltNearbyPoweredStructure
  (params (PoweredStructure :type Primal%20Structure%20Item%20Container%20Object%20Reference))
  (|CallParentFunction PoweredStructure)
  (Class|ArkFrameLogicExpansionInterface|ExpandedPowerGeneratorBuiltNearbyPoweredStructure(Message) (Variables|ArkFrame|System|GetLogicExpansions) PoweredStructure))

(fn BPonContainerActiveHealthDecrease
  (|CallParentFunction)
  (Class|ArkFrameLogicExpansionInterface|ExpandedBPonContainerActiveHealthDecrease(Message) (Variables|ArkFrame|System|GetLogicExpansions)))

(fn BPRefreshedStructureColors
  (|CallParentFunction)
  (Class|ArkFrameLogicExpansionInterface|ExpandedBPRefreshedStructureColors(Message) (Variables|ArkFrame|System|GetLogicExpansions)))

(fn BPPostSetStructureCollisionChannels
  (|CallParentFunction)
  (Class|ArkFrameLogicExpansionInterface|ExpandedBPPostSetStructureCollisionChanels(Message) (Variables|ArkFrame|System|GetLogicExpansions)))

(fn BPPostLoadedfromSaveGame
  (|CallParentFunction)
  (Class|ArkFrameLogicExpansionInterface|ExpandedBPPostLoadedfromSaveGame(Message) (Variables|ArkFrame|System|GetLogicExpansions)))

(fn BPGetInfofromConsumedItemforPlacedStructure
  (params (ItemToConsumed :type Primal%20Item%20Object%20Reference))
  (|CallParentFunction ItemToConsumed)
  (Class|ArkFrameLogicExpansionInterface|ExpandedBPGetInfofromConsumedItemforPlacedStructure(Message) (Variables|ArkFrame|System|GetLogicExpansions) ItemToConsumed))

(fn BPApplyCustomDurabilityonPickup
  (params (pickedup :type Primal%20Item%20Object%20Reference))
  (|CallParentFunction pickedup)
  (Class|ArkFrameLogicExpansionInterface|ExpandedBPApplyCustomDurabilityonPickup(Message) (Variables|ArkFrame|System|GetLogicExpansions) pickedup))

(fn BPHitEffect
  (params (DamageTaken :type Float%20%28single-precision%29) (DamageEvent :type Damage%20Event%20Structure%20%28by%20ref%29) (PawnInstigator :type Pawn%20Object%20Reference) (DamageCauser :type Actor%20Object%20Reference) (bIsLocalPath :type Boolean) (HitComponent :type Primitive%20Component%20Object%20Reference) (DamageLoc :type Vector :default "0, 0, 0") (HitNormal :type Rotator :default "0, 0, 0"))
  (|CallParentFunction DamageTaken DamageEvent PawnInstigator DamageCauser bIsLocalPath HitComponent DamageLoc HitNormal)
  (Class|ArkFrameLogicExpansionInterface|ExpandedBPHitEffect(Message) (Variables|ArkFrame|System|GetLogicExpansions) DamageTaken DamageEvent PawnInstigator DamageCauser bIsLocalPath HitComponent DamageLoc HitNormal)
  (return))

(fn DrawBasicFloatingHUD
  (params (ForHUD :type HUD%20Object%20Reference))
  (|CallParentFunction ForHUD)
  (Class|ArkFrameLogicExpansionInterface|ExpandedDrawBasicFloatingHUD(Message) (Variables|ArkFrame|System|GetLogicExpansions) ForHUD))

(fn BPTryMultiUse
  (params (ForPC :type Player%20Controller%20Object%20Reference) (UseIndex :type Integer))
  (bind _variable (|TemporaryVariable))
  (bind _returnvalue (|CallParentFunction ForPC UseIndex))
  (Utilities|Array|Add _variable _returnvalue)
  (for _array_element (Variables|ArkFrame|System|GetLogicExpansions)
    (bind _breturnvalue (Class|ArkFrameLogicExpansionInterface|ExpandedBPTryMultiUse(Message) _array_element ForPC UseIndex))
    (Utilities|Array|Add _variable _breturnvalue))
  (return (Utilities|Array|ContainsItem _variable true)))

(fn BPPreInitializeComponents
  (|CallParentFunction)
  (Class|ArkFrameLogicExpansionInterface|ExpandedBPPreInitializeComponents(Message) (Variables|ArkFrame|System|GetLogicExpansions)))

(fn BPPostInitializeComponents
  (|CallParentFunction)
  (Class|ArkFrameLogicExpansionInterface|ExpandedBPPostInitializeComponents(Message) (Variables|ArkFrame|System|GetLogicExpansions)))

(fn BPInventoryItemUsed
  (params (InventoryItemObject :type Object%20Object%20Reference))
  (|CallParentFunction InventoryItemObject)
  (Class|ArkFrameLogicExpansionInterface|ExpandedBPInventoryItemUsed(Message) (Variables|ArkFrame|System|GetLogicExpansions) InventoryItemObject))

(fn BPInventoryItemDropped
  (params (InventoryItemObject :type Object%20Object%20Reference))
  (|CallParentFunction InventoryItemObject)
  (Class|ArkFrameLogicExpansionInterface|ExpandedBPInventoryItemDropped(Message) (Variables|ArkFrame|System|GetLogicExpansions) InventoryItemObject))

(fn BPGetMultiUseEntries
  (params (ForPC :type Player%20Controller%20Object%20Reference) (MultiUseEntries :type Array%20of%20Multi%20Use%20Entry%20Structures))
  (LocalVariables|SetL_MultiUseBuffer MultiUseEntries)
  (Utilities|FlowControl|Sequence
    (:then_0
      ;[1 1 1] Reserve default MultiUse Indices (Fully executes only once)
      (if (not (Variables|ArkFrame|System|GetbIsMultiUseReservationComplete))
        (for _array_element (LocalVariables|GetL_MultiUseBuffer)
          (Utilities|Array|Add (Variables|ArkFrame|System|GetMultiUseReservedIndices) (.UseIndex (Utilities|Struct|BreakMultiUseEntry _array_element))))
        (Variables|ArkFrame|System|SetbIsMultiUseReservationComplete true)))
    (:then_1
      (for _array_element_2 (Variables|ArkFrame|System|GetLogicExpansions)
        (Utilities|FlowControl|Sequence
          (:then_0
            ;[1 1 1] Reserve MultiUse Indices with the logic expansion (Fully executes only once)
            (bind _outadditionalmultiusereservations (Default|ReserveMultiUseIndices _array_element_2 (Variables|ArkFrame|System|GetMultiUseReservedIndices)))
            (Utilities|Array|AppendArray (Variables|ArkFrame|System|GetMultiUseReservedIndices) _outadditionalmultiusereservations))
          (:then_1
            ;[1 1 1] Get MultiUse Entries from logic expansion (At this point the logic expansion has an array populated with it's own reserved indices
            (bind _returnvalue (Class|ArkFrameLogicExpansionInterface|ExpandedBPGetMultiUseEntries(Message) _array_element_2 ForPC (LocalVariables|GetL_MultiUseBuffer)))
            (Utilities|Array|AppendArray (LocalVariables|GetL_MultiUseBuffer) _returnvalue))))
      (return (LocalVariables|GetL_MultiUseBuffer)))))

(fn BPClientDoMultiUse
  (params (ForPC :type Player%20Controller%20Object%20Reference) (ClientUseIndex :type Integer))
  (|CallParentFunction ForPC ClientUseIndex)
  (Class|ArkFrameLogicExpansionInterface|ExpandedBPClientDoMultiUse(Message) (Variables|ArkFrame|System|GetLogicExpansions) ForPC ClientUseIndex))

(fn BPChangedActorTeam
  (|CallParentFunction)
  (Class|ArkFrameLogicExpansionInterface|ExpandedBPChangedActorTeam(Message) (Variables|ArkFrame|System|GetLogicExpansions)))

(fn BPAttachedRootComponent
  (|CallParentFunction)
  (Class|ArkFrameLogicExpansionInterface|ExpandedBPAttachedRootComponent(Message) (Variables|ArkFrame|System|GetLogicExpansions)))

(fn BPTriggerStasisEvent
  (|CallParentFunction)
  (Class|ArkFrameLogicExpansionInterface|ExpandedBPTriggerStasisEvent(Message) (Variables|ArkFrame|System|GetLogicExpansions)))

(fn BlueprintDrawHUD
  (params (HUD :type Shooter%20HUD%20Object%20Reference) (CenterX :type Float%20%28single-precision%29) (CenterY :type Float%20%28single-precision%29))
  (|CallParentFunction HUD CenterX CenterY)
  (Class|ArkFrameLogicExpansionInterface|ExpandedBlueprintDrawHUD(Message) (Variables|ArkFrame|System|GetLogicExpansions) HUD CenterX CenterY))

(fn ReceiveRadialDamage
  (params (DamageReceived :type Float%20%28single-precision%29) (DamageType :type Damage%20Type%20Object%20Reference) (Origin :type Vector :default "0, 0, 0") (HitInfo :type Hit%20Result%20Structure%20%28by%20ref%29) (InstigatedBy :type Controller%20Object%20Reference) (DamageCauser :type Actor%20Object%20Reference))
  (|CallParentFunction DamageReceived DamageType Origin HitInfo InstigatedBy DamageCauser)
  (Class|ArkFrameLogicExpansionInterface|ExpandedRadialDamage(Message) (Variables|ArkFrame|System|GetLogicExpansions) DamageReceived DamageType Origin HitInfo InstigatedBy DamageCauser)
  (return))

(fn ReceivePointDamage
  (params (Damage :type Float%20%28single-precision%29) (DamageType :type Damage%20Type%20Object%20Reference) (HitLocation :type Vector :default "0, 0, 0") (HitNormal :type Vector :default "0, 0, 0") (HitComponent :type Primitive%20Component%20Object%20Reference) (BoneName :type Name :default "None") (ShotFromDirection :type Vector :default "0, 0, 0") (InstigatedBy :type Controller%20Object%20Reference) (DamageCauser :type Actor%20Object%20Reference))
  (|CallParentFunction Damage DamageType HitLocation HitNormal HitComponent BoneName ShotFromDirection InstigatedBy DamageCauser)
  (Class|ArkFrameLogicExpansionInterface|ExpandedPointDamage(Message) (Variables|ArkFrame|System|GetLogicExpansions) Damage DamageType HitLocation HitNormal HitComponent BoneName ShotFromDirection InstigatedBy DamageCauser))

(fn ReceiveAnyDamage
  (params (Damage :type Float%20%28single-precision%29) (DamageType :type Damage%20Type%20Object%20Reference) (InstigatedBy :type Controller%20Object%20Reference) (DamageCauser :type Actor%20Object%20Reference))
  (|CallParentFunction Damage DamageType InstigatedBy DamageCauser)
  (Class|ArkFrameLogicExpansionInterface|ExpandedAnyDamage(Message) (Variables|ArkFrame|System|GetLogicExpansions) Damage DamageType InstigatedBy DamageCauser))

(fn RecieveMatineeUpdated
  (|CallParentFunction)
  (Class|ArkFrameLogicExpansionInterface|ExpandedRecieveMatineeUpdated(Message) (Variables|ArkFrame|System|GetLogicExpansions)))

(fn K2onEndViewTarget
  (params (PC :type Player%20Controller%20Object%20Reference))
  (|CallParentFunction PC)
  (Class|ArkFrameLogicExpansionInterface|ExpandedonEndViewTarget(Message) (Variables|ArkFrame|System|GetLogicExpansions) PC))

(fn K2onBecomeViewTarget
  (params (PC :type Player%20Controller%20Object%20Reference))
  (|CallParentFunction PC)
  (Class|ArkFrameLogicExpansionInterface|ExpandedonBecomeViewTarget(Message) (Variables|ArkFrame|System|GetLogicExpansions) PC))

(fn ReceiveHit
  (params (MyComp :type Primitive%20Component%20Object%20Reference) (Other :type Actor%20Object%20Reference) (OtherComp :type Primitive%20Component%20Object%20Reference) (bSelfMoved :type Boolean) (HitLocation :type Vector :default "0, 0, 0") (HitNormal :type Vector :default "0, 0, 0") (NormalImpulse :type Vector :default "0, 0, 0") (Hit :type Hit%20Result%20Structure%20%28by%20ref%29))
  (|CallParentFunction MyComp Other OtherComp bSelfMoved HitLocation HitNormal NormalImpulse Hit)
  (Class|ArkFrameLogicExpansionInterface|ExpandedHit(Message) (Variables|ArkFrame|System|GetLogicExpansions) MyComp Other OtherComp bSelfMoved HitLocation HitNormal NormalImpulse Hit)
  (return))

(fn ReceiveActorEndOverlap
  (params (OtherActor :type Actor%20Object%20Reference))
  (|CallParentFunction OtherActor)
  (Class|ArkFrameLogicExpansionInterface|ExpandedActorEndOverlap(Message) (Variables|ArkFrame|System|GetLogicExpansions) OtherActor))

(fn ReceiveActorBeginOverlap
  (params (OtherActor :type Actor%20Object%20Reference))
  (|CallParentFunction OtherActor)
  (Class|ArkFrameLogicExpansionInterface|ExpandedActorBeginOverlap(Message) (Variables|ArkFrame|System|GetLogicExpansions) OtherActor))

(fn BPNotifyInventoryItemChange
  (params (bIsItemAdd :type Boolean) (theItem :type Primal%20Item%20Object%20Reference) (bEquipItem :type Boolean))
  (|CallParentFunction bIsItemAdd theItem bEquipItem)
  (Class|ArkFrameLogicExpansionInterface|ExpandedBPNotifyInventoryItemChange(Message) (Variables|ArkFrame|System|GetLogicExpansions) bIsItemAdd theItem bEquipItem))

(fn BPContainerDeactivated
  (|CallParentFunction)
  (Class|ArkFrameLogicExpansionInterface|ExpandedBPContainerDeactivated(Message) (Variables|ArkFrame|System|GetLogicExpansions)))

(fn BPContainerActivated
  (|CallParentFunction)
  (Class|ArkFrameLogicExpansionInterface|ExpandedBPContainerActivated(Message) (Variables|ArkFrame|System|GetLogicExpansions)))