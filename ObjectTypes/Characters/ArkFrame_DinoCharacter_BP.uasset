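; ArkFrame base dino character that lets mods attach logic expansion objects to creature behavior.
; On server BeginPlay it gets expansion templates from the game mode, retrying until ArkFrame is ready, then constructs them.
; Templates and session ID are cached on the class default object so later instances skip the request.
; Overridden dino events call the parent, then forward to every expansion; multi-use merges entries and reserves indices.
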(event Custom|Delayed_GetNegotiatorData
  ;[1 1 1] On timer tick, check to see if the CDO has already been updated first
  (bind _returnvalue (Class|VictoryCore|GetClassDefaultObject (Utilities|GetClass self)))
  (bind _asarkframe_dinocharacter_bp_c (Utilities|Casting|CastToArkFrame_DinoCharacter_BP _returnvalue))
  (if (== (Variables|ArkFrame_DinoCharacter_BP_C|GetCDO_Session_ID _asarkframe_dinocharacter_bp_c) (CallFunction|GetArkFrameSessionID))
    (Variables|ArkFrame|System|SetLogicExpansionTemplates (Variables|ArkFrame_DinoCharacter_BP_C|GetLogicExpansionTemplates _asarkframe_dinocharacter_bp_c))
    (Variables|ArkFrame|System|SetCDO_Session_ID (Variables|ArkFrame_DinoCharacter_BP_C|GetCDO_Session_ID _asarkframe_dinocharacter_bp_c))
    (CallFunction|BuildModExtensionObjects)
    (else
      ;[1 1 1] if not, Make sure ArkFrame is ready
      (if (CallFunction|CheckArkFrameReadiness)
        ;[1 1 1] Request data from the Arkframe sytem, and set the CDO data as well
        (Utilities|Time|ClearTimerbyFunctionName 0 "Delayed_GetNegotiatorData")
        (bind _logicexpansiontemplates (Class|ArkFrameGameModeInterface|GetLogicExpansions(Message) (Game|GetGameMode) (Variables|ArkFrame|GetUniqueName) (Variables|ArkFrame|GetDescriptiveTags)))
        (Variables|ArkFrame|System|SetLogicExpansionTemplates _logicexpansiontemplates)
        (Variables|ArkFrame|System|SetCDO_Session_ID (CallFunction|GetArkFrameSessionID))
        (Utilities|FlowControl|Sequence
          (:then_0
            (bind _returnvalue_2 (Class|VictoryCore|GetClassDefaultObject (Utilities|GetClass self)))
            (bind _asarkframe_dinocharacter_bp_c_2 (Utilities|Casting|CastToArkFrame_DinoCharacter_BP _returnvalue_2))
            (Variables|ArkFrame_DinoCharacter_BP_C|SetLogicExpansionTemplates _asarkframe_dinocharacter_bp_c_2 (Variables|ArkFrame|System|GetLogicExpansionTemplates))
            (Variables|ArkFrame_DinoCharacter_BP_C|SetCDO_Session_ID _asarkframe_dinocharacter_bp_c_2 (Variables|ArkFrame|System|GetCDO_Session_ID)))
          (:then_1
            (CallFunction|BuildModExtensionObjects)))))))

(event Custom|BuildModExtensionObjects
  ;[1 1 1] Generate mod related sub-objects
  (CallFunction|ConstructLogicExpansions (Variables|ArkFrame|System|GetLogicExpansionTemplates) (Variables|ArkFrame|System|GetLogicExpansions) self)
  (Networking|ForceNetUpdate))

(event EventBeginPlay
  ;[1 1 1] Check for if this object was generated from a current CDO
  (|CallParentFunction)
  (Utilities|FlowControl|Delay 0.2)
  (Networking|SwitchHasAuthority
    (:Authority
      (if (== (Variables|ArkFrame|System|GetCDO_Session_ID) (CallFunction|GetArkFrameSessionID))
        (CallFunction|BuildModExtensionObjects)
        (else
          ;[1 1 1] If not then check if the CDO has already been updated for this session
          (bind _returnvalue (Class|VictoryCore|GetClassDefaultObject (Utilities|GetClass self)))
          (bind _asarkframe_dinocharacter_bp_c (Utilities|Casting|CastToArkFrame_DinoCharacter_BP _returnvalue))
          (if (== (Variables|ArkFrame_DinoCharacter_BP_C|GetCDO_Session_ID _asarkframe_dinocharacter_bp_c) (CallFunction|GetArkFrameSessionID))
            (Variables|ArkFrame|System|SetLogicExpansionTemplates (Variables|ArkFrame_DinoCharacter_BP_C|GetLogicExpansionTemplates _asarkframe_dinocharacter_bp_c))
            (Variables|ArkFrame|System|SetCDO_Session_ID (Variables|ArkFrame_DinoCharacter_BP_C|GetCDO_Session_ID _asarkframe_dinocharacter_bp_c))
            (CallFunction|BuildModExtensionObjects)
            (else
              ;[1 1 1] If not, check if the AF system is ready, otherwise set the retry timer
              (if (CallFunction|CheckArkFrameReadiness)
                ;[1 1 1] Request data from the Arkframe sytem, and set the CDO data as well
                (Utilities|Time|ClearTimerbyFunctionName 0 "Delayed_GetNegotiatorData")
                (bind _logicexpansiontemplates (Class|ArkFrameGameModeInterface|GetLogicExpansions(Message) (Game|GetGameMode) (Variables|ArkFrame|GetUniqueName) (Variables|ArkFrame|GetDescriptiveTags)))
                (Variables|ArkFrame|System|SetLogicExpansionTemplates _logicexpansiontemplates)
                (Variables|ArkFrame|System|SetCDO_Session_ID (CallFunction|GetArkFrameSessionID))
                (Utilities|FlowControl|Sequence
                  (:then_0
                    (bind _returnvalue_2 (Class|VictoryCore|GetClassDefaultObject (Utilities|GetClass self)))
                    (bind _asarkframe_dinocharacter_bp_c_2 (Utilities|Casting|CastToArkFrame_DinoCharacter_BP _returnvalue_2))
                    (Variables|ArkFrame_DinoCharacter_BP_C|SetLogicExpansionTemplates _asarkframe_dinocharacter_bp_c_2 (Variables|ArkFrame|System|GetLogicExpansionTemplates))
                    (Variables|ArkFrame_DinoCharacter_BP_C|SetCDO_Session_ID _asarkframe_dinocharacter_bp_c_2 (Variables|ArkFrame|System|GetCDO_Session_ID)))
                  (:then_1
                    (CallFunction|BuildModExtensionObjects)))
                (else
                  (Utilities|Time|SetTimerbyFunctionName 0 "Delayed_GetNegotiatorData" 0.5 true))))))))))

(fn ConstructionScript
  (|CallParentFunction))

(fn RidingTick
  (|CallParentFunction)
  (Class|ArkFrameLogicExpansionInterface|ExpandedRidingTick(Message) (Variables|ArkFrame|System|GetLogicExpansions)))

(fn BSetupDinoTameable
  (|CallParentFunction)
  (Class|ArkFrameLogicExpansionInterface|ExpandedBPSetupDinoTamable(Message) (Variables|ArkFrame|System|GetLogicExpansions)))

(fn BPUntamedConsumeFoodItem
  (params (foodItem :type Primal%20Item%20Object%20Reference))
  (|CallParentFunction foodItem)
  (Class|ArkFrameLogicExpansionInterface|ExpandedBPUntamedConsumeFoodItem(Message) (Variables|ArkFrame|System|GetLogicExpansions) foodItem))

(fn BPUnstasis
  (|CallParentFunction)
  (Class|ArkFrameLogicExpansionInterface|ExpandedBPUnstasis(Message) (Variables|ArkFrame|System|GetLogicExpansions)))

(fn BPUnsetupDinoTameable
  (|CallParentFunction)
  (Class|ArkFrameLogicExpansionInterface|ExpandedBPUnsetupDinoTamable(Message) (Variables|ArkFrame|System|GetLogicExpansions)))

(fn BPSetupTamed
  (params (bWasJustTamed :type Boolean))
  (|CallParentFunction bWasJustTamed)
  (Class|ArkFrameLogicExpansionInterface|ExpandedBPSetupTamed(Message) (Variables|ArkFrame|System|GetLogicExpansions) bWasJustTamed))

(fn BPSentKilledNotification
  (params (ToPC :type Shooter%20Player%20Controller%20Object%20Reference))
  (|CallParentFunction ToPC)
  (Class|ArkFrameLogicExpansionInterface|ExpandedBPSentKilledNotification(Message) (Variables|ArkFrame|System|GetLogicExpansions) ToPC))

(fn BPNotifyStructurePlacedNearby
  (params (NewStructure :type Primal%20Structure%20Object%20Reference))
  (|CallParentFunction NewStructure)
  (Class|ArkFrameLogicExpansionInterface|ExpandedBPNotifyStructurePlacedNearby(Message) (Variables|ArkFrame|System|GetLogicExpansions) NewStructure))

(fn BPDoAttack
  (params (AttackIndex :type Integer))
  (|CallParentFunction AttackIndex)
  (Class|ArkFrameLogicExpansionInterface|ExpandedBPDoAttack(Message) (Variables|ArkFrame|System|GetLogicExpansions) AttackIndex))

(fn BPDinoPrepareforARKUploading
  (|CallParentFunction)
  (Class|ArkFrameLogicExpansionInterface|ExpandedBPDinoPrepareforARKUploading(Message) (Variables|ArkFrame|System|GetLogicExpansions)))

(fn BPDinoPostBeginPlay
  (|CallParentFunction)
  (Class|ArkFrameLogicExpansionInterface|ExpandedBPDinoPostBeginPlay(Message) (Variables|ArkFrame|System|GetLogicExpansions)))

(fn BPDinoARKDownloadedEnd
  (|CallParentFunction)
  (Class|ArkFrameLogicExpansionInterface|ExpandedBPDinoARKDownloadedEnd(Message) (Variables|ArkFrame|System|GetLogicExpansions)))

(fn BPDinoARKDownloadedBegin
  (|CallParentFunction)
  (Class|ArkFrameLogicExpansionInterface|ExpandedBPDinoARKDownloadedBegin(Message) (Variables|ArkFrame|System|GetLogicExpansions)))

(fn BPDidSetCarriedCharacter
  (params (PreviousCarriedCharacter :type Primal%20Character%20Object%20Reference))
  (|CallParentFunction PreviousCarriedCharacter)
  (Class|ArkFrameLogicExpansionInterface|ExpandedBPDidSetCarriedCharacter(Message) (Variables|ArkFrame|System|GetLogicExpansions) PreviousCarriedCharacter))

(fn BPDidClearCarriedCharacter
  (params (PreviousCarriedCharacter :type Primal%20Character%20Object%20Reference))
  (|CallParentFunction PreviousCarriedCharacter)
  (Class|ArkFrameLogicExpansionInterface|ExpandedBPDidClearCarriedCharacter(Message) (Variables|ArkFrame|System|GetLogicExpansions) PreviousCarriedCharacter))

(fn BPBecomeBaby
  (|CallParentFunction)
  (Class|ArkFrameLogicExpansionInterface|ExpandedBPBecomeBaby(Message) (Variables|ArkFrame|System|GetLogicExpansions)))

(fn BPBecomeAdult
  (|CallParentFunction)
  (Class|ArkFrameLogicExpansionInterface|ExpandedBPBecomeAdult(Message) (Variables|ArkFrame|System|GetLogicExpansions)))

(fn BPTimerServer
  (|CallParentFunction)
  (Class|ArkFrameLogicExpansionInterface|ExpandedBPTimerServer(Message) (Variables|ArkFrame|System|GetLogicExpansions)))

(fn BPTimerNonDedicated
  (|CallParentFunction)
  (Class|ArkFrameLogicExpansionInterface|ExpandedBPTimerNonDedicated(Message) (Variables|ArkFrame|System|GetLogicExpansions)))

(fn BPPostLoadedfromSaveGame
  (|CallParentFunction)
  (Class|ArkFrameLogicExpansionInterface|ExpandedBPPostLoadedfromSaveGame(Message) (Variables|ArkFrame|System|GetLogicExpansions)))

(fn BPonMovementModeChangedNotify
  (|CallParentFunction)
  (Class|ArkFrameLogicExpansionInterface|ExpandedBPonMovementModeChangedNotify(Message) (Variables|ArkFrame|System|GetLogicExpansions)))

(fn BPonAnimPlayedNotify
  (params (AnimMontage :type Anim%20Montage%20Object%20Reference) (InPlayRate :type Float%20%28single-precision%29) (StartSectionName :type Name :default "None") (bReplicate :type Boolean) (bReplicateToOwner :type Boolean) (bForceTickPoseAndServerUpdateMesh :type Boolean) (bForceTickPoseOnServer :type Boolean))
  (|CallParentFunction AnimMontage InPlayRate StartSectionName bReplicate bReplicateToOwner bForceTickPoseAndServerUpdateMesh bForceTickPoseOnServer)
  (Class|ArkFrameLogicExpansionInterface|ExpandedBPonAnimPlayedNotify(Message) (Variables|ArkFrame|System|GetLogicExpansions) AnimMontage InPlayRate StartSectionName bReplicate bReplicateToOwner bForceTickPoseAndServerUpdateMesh bForceTickPoseOnServer))

(fn BPNotifyLevelUp
  (params (ExtraCharacterLevel :type Integer))
  (|CallParentFunction ExtraCharacterLevel)
  (Class|ArkFrameLogicExpansionInterface|ExpandedBPNotifyLevelUp(Message) (Variables|ArkFrame|System|GetLogicExpansions) ExtraCharacterLevel))

(fn BPCharacterUnsleeped
  (|CallParentFunction)
  (Class|ArkFrameLogicExpansionInterface|ExpandedBPCharacterUnsleeped(Message) (Variables|ArkFrame|System|GetLogicExpansions)))

(fn BPCharacterSleeped
  (|CallParentFunction)
  (Class|ArkFrameLogicExpansionInterface|ExpandedBPCharacterSleeped(Message) (Variables|ArkFrame|System|GetLogicExpansions)))

(fn BPAddedAttachmentsforItem
  (params (anItem :type Primal%20Item%20Object%20Reference))
  (|CallParentFunction anItem)
  (Class|ArkFrameLogicExpansionInterface|ExpandedBPAddedAttachmentsforItem(Message) (Variables|ArkFrame|System|GetLogicExpansions) anItem))

(fn OnLaunched
  (params (LaunchVelocity :type Vector :default "0, 0, 0") (bXYOverride :type Boolean) (bZOverride :type Boolean))
  (|CallParentFunction LaunchVelocity bXYOverride bZOverride)
  (Class|ArkFrameLogicExpansionInterface|ExpandedonLaunched(Message) (Variables|ArkFrame|System|GetLogicExpansions) LaunchVelocity bXYOverride bZOverride))

(fn OnLanded
  (params (Hit :type Hit%20Result%20Structure%20%28by%20ref%29))
  (|CallParentFunction Hit)
  (Class|ArkFrameLogicExpansionInterface|ExpandedonLanded(Message) (Variables|ArkFrame|System|GetLogicExpansions) Hit)
  (return))

(fn K2onStartCrouch
  (params (HalfHeightAdjust :type Float%20%28single-precision%29) (ScaledHalfHeightAdjust :type Float%20%28single-precision%29))
  (|CallParentFunction HalfHeightAdjust ScaledHalfHeightAdjust)
  (Class|ArkFrameLogicExpansionInterface|ExpandedonStartCrouch(Message) (Variables|ArkFrame|System|GetLogicExpansions) HalfHeightAdjust ScaledHalfHeightAdjust))

(fn K2onMovementModeChanged
  (params (PrevMovementMode :type EMovementMode%20Enum :default "MOVE_None") (NewMovementMode :type EMovementMode%20Enum :default "MOVE_None") (PrevCustomMode :type Byte :default 0) (NewCustomMode :type Byte :default 0))
  (|CallParentFunction PrevMovementMode NewMovementMode PrevCustomMode NewCustomMode)
  (Class|ArkFrameLogicExpansionInterface|ExpandedonMovementModeChanged(Message) (Variables|ArkFrame|System|GetLogicExpansions) PrevMovementMode NewMovementMode PrevCustomMode NewCustomMode))

(fn K2onEndCrouch
  (params (HalfHeightAdjust :type Float%20%28single-precision%29) (ScaledHalfHeightAdjust :type Float%20%28single-precision%29))
  (|CallParentFunction HalfHeightAdjust ScaledHalfHeightAdjust)
  (Class|ArkFrameLogicExpansionInterface|ExpandedonEndCrouch(Message) (Variables|ArkFrame|System|GetLogicExpansions) HalfHeightAdjust ScaledHalfHeightAdjust))

(fn ReceiveUnpossessed
  (params (OldController :type Controller%20Object%20Reference))
  (|CallParentFunction OldController)
  (Class|ArkFrameLogicExpansionInterface|ExpandedUnpossessed(Message) (Variables|ArkFrame|System|GetLogicExpansions) OldController))

(fn ReceivePossessed
  (params (NewController :type Controller%20Object%20Reference))
  (|CallParentFunction NewController)
  (Class|ArkFrameLogicExpansionInterface|ExpandedPossessed(Message) (Variables|ArkFrame|System|GetLogicExpansions) NewController))

(fn DrawBasicFloatingHUD
  (params (ForHUD :type HUD%20Object%20Reference))
  (|CallParentFunction ForHUD)
  (Class|ArkFrameLogicExpansionInterface|ExpandedDrawBasicFloatingHUD(Message) (Variables|ArkFrame|System|GetLogicExpansions) ForHUD))

(fn BPTryMultiUse
  (params (ForPC :type Player%20Controller%20Object%20Reference) (UseIndex :type Integer))
  (bind _variable (|TemporaryVariable))
  (bind _returnvalue (|CallParentFunction ForPC UseIndex))
  (Utilities|Array|Add _variable _returnvalue)
  (for _array_element (Variables|ArkFrame|System|GetLogicExpansions)
    (bind _breturnvalue (Class|ArkFrameLogicExpansionInterface|ExpandedBPTryMultiUse(Message) _array_element ForPC UseIndex))
    (Utilities|Array|Add _variable _breturnvalue))
  (return (Utilities|Array|ContainsItem _variable true)))

(fn BPPreInitializeComponents
  (|CallParentFunction)
  (Class|ArkFrameLogicExpansionInterface|ExpandedBPPreInitializeComponents(Message) (Variables|ArkFrame|System|GetLogicExpansions)))

(fn BPPostInitializeComponents
  (|CallParentFunction)
  (Class|ArkFrameLogicExpansionInterface|ExpandedBPPostInitializeComponents(Message) (Variables|ArkFrame|System|GetLogicExpansions)))

(fn BPInventoryItemUsed
  (params (InventoryItemObject :type Object%20Object%20Reference))
  (|CallParentFunction InventoryItemObject)
  (Class|ArkFrameLogicExpansionInterface|ExpandedBPInventoryItemUsed(Message) (Variables|ArkFrame|System|GetLogicExpansions) InventoryItemObject))

(fn BPInventoryItemDropped
  (params (InventoryItemObject :type Object%20Object%20Reference))
  (|CallParentFunction InventoryItemObject)
  (Class|ArkFrameLogicExpansionInterface|ExpandedBPInventoryItemDropped(Message) (Variables|ArkFrame|System|GetLogicExpansions) InventoryItemObject))

(fn BPGetMultiUseEntries
  (params (ForPC :type Player%20Controller%20Object%20Reference) (MultiUseEntries :type Array%20of%20Multi%20Use%20Entry%20Structures))
  (bind _returnvalue (|CallParentFunction ForPC MultiUseEntries))
  (LocalVariables|SetL_MultiUseBuffer _returnvalue)
  (Utilities|FlowControl|Sequence
    (:then_0
      ;[1 1 1] Reserve default MultiUse Indices (Fully executes only once)
      (if (not (Variables|ArkFrame|System|GetbIsMultiUseReservationComplete))
        (for _array_element (LocalVariables|GetL_MultiUseBuffer)
          (Utilities|Array|Add (Variables|ArkFrame|System|GetMultiUseReservedIndices) (.UseIndex (Utilities|Struct|BreakMultiUseEntry _array_element))))
        (Variables|ArkFrame|System|SetbIsMultiUseReservationComplete true)))
    (:then_1
      (for _array_element_2 (Variables|ArkFrame|System|GetLogicExpansions)
        (Utilities|FlowControl|Sequence
          (:then_0
            ;[1 1 1] Reserve MultiUse Indices with the logic expansion (Fully executes only once)
            (bind _outadditionalmultiusereservations (Default|ReserveMultiUseIndices _array_element_2 (Variables|ArkFrame|System|GetMultiUseReservedIndices)))
            (Utilities|Array|AppendArray (Variables|ArkFrame|System|GetMultiUseReservedIndices) _outadditionalmultiusereservations))
          (:then_1
            ;[1 1 1] Get MultiUse Entries from logic expansion (At this point the logic expansion has an array populated with it's own reserved indices
            (bind _returnvalue_2 (Class|ArkFrameLogicExpansionInterface|ExpandedBPGetMultiUseEntries(Message) _array_element_2 ForPC (LocalVariables|GetL_MultiUseBuffer)))
            (Utilities|Array|AppendArray (LocalVariables|GetL_MultiUseBuffer) _returnvalue_2))))
      (return (LocalVariables|GetL_MultiUseBuffer)))))

(fn BPChangedActorTeam
  (|CallParentFunction)
  (Class|ArkFrameLogicExpansionInterface|ExpandedBPChangedActorTeam(Message) (Variables|ArkFrame|System|GetLogicExpansions)))

(fn BPAttachedRootComponent
  (|CallParentFunction)
  (Class|ArkFrameLogicExpansionInterface|ExpandedBPAttachedRootComponent(Message) (Variables|ArkFrame|System|GetLogicExpansions)))

(fn BPonTamedProcessOrder
  (params (FromCharacter :type Primal%20Character%20Object%20Reference) (OrderType :type EDinoTamedOrder%20Enum :default "SetAggressionPassive") (bForce :type Boolean) (enemyTarget :type Actor%20Object%20Reference))
  (|CallParentFunction FromCharacter OrderType bForce enemyTarget)
  (Class|ArkFrameLogicExpansionInterface|ExpandedBPonTamedProcessOrder(Message) (Variables|ArkFrame|System|GetLogicExpansions) FromCharacter OrderType bForce enemyTarget))

(fn BPDoHarvestAttack
  (params (harvestIndex :type Integer))
  (|CallParentFunction harvestIndex)
  (Class|ArkFrameLogicExpansionInterface|ExpandedBPDoHarvestAttack(Message) (Variables|ArkFrame|System|GetLogicExpansions) harvestIndex))

(fn InterruptLatching
  (|CallParentFunction)
  (Class|ArkFrameLogicExpansionInterface|ExpandedInterruptLatching(Message) (Variables|ArkFrame|System|GetLogicExpansions)))

(fn HandleMountedDinoAction
  (params (PC :type Shooter%20Player%20Controller%20Object%20Reference))
  (|CallParentFunction PC)
  (Class|ArkFrameLogicExpansionInterface|ExpandedHandleMountedDinoAction(Message) (Variables|ArkFrame|System|GetLogicExpansions) PC))

(fn BPNotifySetRider
  (params (RiderSetting :type Shooter%20Character%20Object%20Reference))
  (|CallParentFunction RiderSetting)
  (Class|ArkFrameLogicExpansionInterface|ExpandedBPNotifySetRider(Message) (Variables|ArkFrame|System|GetLogicExpansions) RiderSetting))

(fn BPNotifyClearRider
  (params (RiderClearing :type Shooter%20Character%20Object%20Reference))
  (|CallParentFunction RiderClearing)
  (Class|ArkFrameLogicExpansionInterface|ExpandedBPNotifyClearRider(Message) (Variables|ArkFrame|System|GetLogicExpansions) RiderClearing))

(fn BPKilledSomethingEvent
  (params (killedTarget :type Primal%20Character%20Object%20Reference))
  (|CallParentFunction killedTarget)
  (Class|ArkFrameLogicExpansionInterface|ExpandedBPKilledSomethingEvent(Message) (Variables|ArkFrame|System|GetLogicExpansions) killedTarget))

(fn BPFedWakingTameEvent
  (params (ForPC :type Player%20Controller%20Object%20Reference))
  (|CallParentFunction ForPC)
  (Class|ArkFrameLogicExpansionInterface|ExpandedBPFedWakingTameEvent(Message) (Variables|ArkFrame|System|GetLogicExpansions) ForPC))

(fn BlueprintTamedTick
  (|CallParentFunction)
  (Class|ArkFrameLogicExpansionInterface|ExpandedBlueprintTamedTick(Message) (Variables|ArkFrame|System|GetLogicExpansions)))

(fn DinoShoulderMountedLaunch
  (params (launchDir :type Vector :default "0, 0, 0") (throwingCharacter :type Shooter%20Character%20Object%20Reference))
  (|CallParentFunction launchDir throwingCharacter)
  (Class|ArkFrameLogicExpansionInterface|ExpandedDinoShoulderMountedLaunch(Message) (Variables|ArkFrame|System|GetLogicExpansions) launchDir throwingCharacter))

(fn BPonSetMountedDino
  (|CallParentFunction)
  (Class|ArkFrameLogicExpansionInterface|ExpandedBPonSetMountedDino(Message) (Variables|ArkFrame|System|GetLogicExpansions)))

(fn BPonClearMountedDino
  (|CallParentFunction)
  (Class|ArkFrameLogicExpansionInterface|ExpandedBPonClearMountedDino(Message) (Variables|ArkFrame|System|GetLogicExpansions)))

(fn BlueprintPlayDying
  (params (KillingDamage :type Float%20%28single-precision%29) (DamageEvent :type Damage%20Event%20Structure%20%28by%20ref%29) (InstigatingPawn :type Pawn%20Object%20Reference) (DamageCauser :type Actor%20Object%20Reference))
  (|CallParentFunction KillingDamage DamageEvent InstigatingPawn DamageCauser)
  (Class|ArkFrameLogicExpansionInterface|ExpandedBlueprintPlayDying(Message) (Variables|ArkFrame|System|GetLogicExpansions) KillingDamage DamageEvent InstigatingPawn DamageCauser)
  (return))

(fn OnWalkingOffLedge
  (|CallParentFunction)
  (Class|ArkFrameLogicExpansionInterface|ExpandedonWalkedOffLedge(Message) (Variables|ArkFrame|System|GetLogicExpansions)))

(fn OnJumped
  (|CallParentFunction)
  (Class|ArkFrameLogicExpansionInterface|ExpandedonJumped(Message) (Variables|ArkFrame|System|GetLogicExpansions)))

(fn BPNotifyBumpedPawn
  (params (BumpedPawn :type Primal%20Character%20Object%20Reference))
  (|CallParentFunction BumpedPawn)
  (Class|ArkFrameLogicExpansionInterface|ExpandedNotifyBumpedPawn(Message) (Variables|ArkFrame|System|GetLogicExpansions) BumpedPawn))

(fn BPNotifyBumpedbyPawn
  (params (ByPawn :type Primal%20Character%20Object%20Reference))
  (|CallParentFunction ByPawn)
  (Class|ArkFrameLogicExpansionInterface|ExpandedNotifyBumpedbyPawn(Message) (Variables|ArkFrame|System|GetLogicExpansions) ByPawn))

(fn BPonJumpReleased
  (|CallParentFunction)
  (Class|ArkFrameLogicExpansionInterface|ExpandedBPonJumpReleased(Message) (Variables|ArkFrame|System|GetLogicExpansions)))

(fn BPonJumpPressed
  (|CallParentFunction)
  (Class|ArkFrameLogicExpansionInterface|ExpandedBPonJumpPressed(Message) (Variables|ArkFrame|System|GetLogicExpansions)))

(fn BlueprintDrawFloatingHUD
  (params (HUD :type Shooter%20HUD%20Object%20Reference) (CenterX :type Float%20%28single-precision%29) (CenterY :type Float%20%28single-precision%29) (DrawScale :type Float%20%28single-precision%29))
  (|CallParentFunction HUD CenterX CenterY DrawScale)
  (Class|ArkFrameLogicExpansionInterface|ExpandedBlueprintDrawFloatingHUD(Message) (Variables|ArkFrame|System|GetLogicExpansions) HUD CenterX CenterY DrawScale))

(fn ReceiveRadialDamage
  (params (DamageReceived :type Float%20%28single-precision%29) (DamageType :type Damage%20Type%20Object%20Reference) (Origin :type Vector :default "0, 0, 0") (HitInfo :type Hit%20Result%20Structure%20%28by%20ref%29) (InstigatedBy :type Controller%20Object%20Reference) (DamageCauser :type Actor%20Object%20Reference))
  (|CallParentFunction DamageReceived DamageType Origin HitInfo InstigatedBy DamageCauser)
  (Class|ArkFrameLogicExpansionInterface|ExpandedRadialDamage(Message) (Variables|ArkFrame|System|GetLogicExpansions) DamageReceived DamageType Origin HitInfo InstigatedBy DamageCauser)
  (return))

(fn ReceivePointDamage
  (params (Damage :type Float%20%28single-precision%29) (DamageType :type Damage%20Type%20Object%20Reference) (HitLocation :type Vector :default "0, 0, 0") (HitNormal :type Vector :default "0, 0, 0") (HitComponent :type Primitive%20Component%20Object%20Reference) (BoneName :type Name :default "None") (ShotFromDirection :type Vector :default "0, 0, 0") (InstigatedBy :type Controller%20Object%20Reference) (DamageCauser :type Actor%20Object%20Reference))
  (|CallParentFunction Damage DamageType HitLocation HitNormal HitComponent BoneName ShotFromDirection InstigatedBy DamageCauser)
  (Class|ArkFrameLogicExpansionInterface|ExpandedPointDamage(Message) (Variables|ArkFrame|System|GetLogicExpansions) Damage DamageType HitLocation HitNormal HitComponent BoneName ShotFromDirection InstigatedBy DamageCauser))

(fn ReceiveAnyDamage
  (params (Damage :type Float%20%28single-precision%29) (DamageType :type Damage%20Type%20Object%20Reference) (InstigatedBy :type Controller%20Object%20Reference) (DamageCauser :type Actor%20Object%20Reference))
  (|CallParentFunction Damage DamageType InstigatedBy DamageCauser)
  (Class|ArkFrameLogicExpansionInterface|ExpandedAnyDamage(Message) (Variables|ArkFrame|System|GetLogicExpansions) Damage DamageType InstigatedBy DamageCauser))

(fn BPTriggerStasisEvent
  (|CallParentFunction)
  (Class|ArkFrameLogicExpansionInterface|ExpandedBPTriggerStasisEvent(Message) (Variables|ArkFrame|System|GetLogicExpansions)))

(fn BlueprintAnimNotifyCustomEvent
  (params (CustomEventName :type Name :default "None") (MeshComp :type Skeletal%20Mesh%20Component%20Object%20Reference) (Animation :type Anim%20Sequence%20Base%20Object%20Reference) (AnimNotifyObject :type Anim%20Notify%20Object%20Reference))
  (|CallParentFunction CustomEventName MeshComp Animation AnimNotifyObject)
  (Class|ArkFrameLogicExpansionInterface|ExpandedBlueprintAnimNotifyCustomEvent(Message) (Variables|ArkFrame|System|GetLogicExpansions) CustomEventName MeshComp Animation AnimNotifyObject))

(fn RecieveMatineeUpdated
  (|CallParentFunction)
  (Class|ArkFrameLogicExpansionInterface|ExpandedRecieveMatineeUpdated(Message) (Variables|ArkFrame|System|GetLogicExpansions)))

(fn ReceiveHit
  (params (MyComp :type Primitive%20Component%20Object%20Reference) (Other :type Actor%20Object%20Reference) (OtherComp :type Primitive%20Component%20Object%20Reference) (bSelfMoved :type Boolean) (HitLocation :type Vector :default "0, 0, 0") (HitNormal :type Vector :default "0, 0, 0") (NormalImpulse :type Vector :default "0, 0, 0") (Hit :type Hit%20Result%20Structure%20%28by%20ref%29))
  (|CallParentFunction MyComp Other OtherComp bSelfMoved HitLocation HitNormal NormalImpulse Hit)
  (Class|ArkFrameLogicExpansionInterface|ExpandedHit(Message) (Variables|ArkFrame|System|GetLogicExpansions) MyComp Other OtherComp bSelfMoved HitLocation HitNormal NormalImpulse Hit)
  (return))

(fn ReceiveActorEndOverlap
  (params (OtherActor :type Actor%20Object%20Reference))
  (|CallParentFunction OtherActor)
  (Class|ArkFrameLogicExpansionInterface|ExpandedActorEndOverlap(Message) (Variables|ArkFrame|System|GetLogicExpansions) OtherActor))

(fn ReceiveActorBeginOverlap
  (params (OtherActor :type Actor%20Object%20Reference))
  (|CallParentFunction OtherActor)
  (Class|ArkFrameLogicExpansionInterface|ExpandedActorBeginOverlap(Message) (Variables|ArkFrame|System|GetLogicExpansions) OtherActor))

(fn K2onEndViewTarget
  (params (PC :type Player%20Controller%20Object%20Reference))
  (|CallParentFunction PC)
  (Class|ArkFrameLogicExpansionInterface|ExpandedonEndViewTarget(Message) (Variables|ArkFrame|System|GetLogicExpansions) PC))

(fn K2onBecomeViewTarget
  (params (PC :type Player%20Controller%20Object%20Reference))
  (|CallParentFunction PC)
  (Class|ArkFrameLogicExpansionInterface|ExpandedonBecomeViewTarget(Message) (Variables|ArkFrame|System|GetLogicExpansions) PC))

(fn BPClientDoMultiUse
  (params (ForPC :type Player%20Controller%20Object%20Reference) (ClientUseIndex :type Integer))
  (|CallParentFunction ForPC ClientUseIndex)
  (Class|ArkFrameLogicExpansionInterface|ExpandedBPClientDoMultiUse(Message) (Variables|ArkFrame|System|GetLogicExpansions) ForPC ClientUseIndex))