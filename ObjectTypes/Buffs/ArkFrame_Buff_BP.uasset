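; ArkFrame base buff that lets mods extend buff behavior through logic expansion objects.
; Authority BeginPlay builds expansions from templates when the session ID is current; its CDO-check and retry-timer fallback is disconnected.
; Delayed_GetNegotiatorData takes templates from the class default object or ArkFrame manager, caching fetched ones on the CDO per session.
; Buff, damage, HUD, collision and lifecycle overrides call their parent, then forward to the expansions.
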(event Custom|Delayed_GetNegotiatorData
  ;[1 1 1] On timer tick, check to see if the CDO has already been updated first
  (bind _returnvalue (Class|VictoryCore|GetClassDefaultObject (Utilities|GetClass self)))
  (bind _asarkframe_buff_bp_c (Utilities|Casting|CastToArkFrame_Buff_BP _returnvalue))
  (if (== (Variables|ArkFrame_Buff_BP_C|GetCDO_Session_ID _asarkframe_buff_bp_c) (CallFunction|GetArkFrameSessionID))
    (Variables|ArkFrame|System|SetLogicExpansionTemplates (Variables|ArkFrame_Buff_BP_C|GetLogicExpansionTemplates _asarkframe_buff_bp_c))
    (Variables|ArkFrame|System|SetCDO_Session_ID (Variables|ArkFrame_Buff_BP_C|GetCDO_Session_ID _asarkframe_buff_bp_c))
    (CallFunction|BuildModExtensionObjects)
    (else
      ;[1 1 1] if not, Make sure ArkFrame is ready
      (if (CallFunction|CheckArkFrameReadiness)
        ;[1 1 1] Request data from the Arkframe sytem, and set the CDO data as well
        (Utilities|Time|ClearTimerbyFunctionName 0 "Delayed_GetNegotiatorData")
        (bind _logicexpansiontemplates (Class|ArkFrameManagerInterface|GetLogicExpansions(Message) (CallFunction|GetArkFrameManager) (Variables|ArkFrame|GetUniqueName) (Variables|ArkFrame|GetDescriptiveTags)))
        (Variables|ArkFrame|System|SetLogicExpansionTemplates _logicexpansiontemplates)
        (Variables|ArkFrame|System|SetCDO_Session_ID (CallFunction|GetArkFrameSessionID))
        (Utilities|FlowControl|Sequence
          (:then_0
            (bind _returnvalue_2 (Class|VictoryCore|GetClassDefaultObject (Utilities|GetClass self)))
            (bind _asarkframe_buff_bp_c_2 (Utilities|Casting|CastToArkFrame_Buff_BP _returnvalue_2))
            (Variables|ArkFrame_Buff_BP_C|SetLogicExpansionTemplates _asarkframe_buff_bp_c_2 (Variables|ArkFrame|System|GetLogicExpansionTemplates))
            (Variables|ArkFrame_Buff_BP_C|SetCDO_Session_ID _asarkframe_buff_bp_c_2 (Variables|ArkFrame|System|GetCDO_Session_ID)))
          (:then_1
            (CallFunction|BuildModExtensionObjects)))))))

(event Custom|BuildModExtensionObjects
  ;[1 1 1] Generate mod related sub-objects
  (CallFunction|ConstructLogicExpansions (Variables|ArkFrame|System|GetLogicExpansionTemplates) (Variables|ArkFrame|System|GetLogicExpansions) self)
  (Networking|ForceNetUpdate))

(event EventBeginPlay
  ;[1 1 1] Check for if this object was generated from a current CDO
  (|CallParentFunction)
  (Utilities|FlowControl|Delay 0.2)
  (Networking|SwitchHasAuthority
    (:Authority
      (if (== (Variables|ArkFrame|System|GetCDO_Session_ID) (CallFunction|GetArkFrameSessionID))
        (CallFunction|BuildModExtensionObjects)
        (else
          ;[1 1 1] If not then check if the CDO has already been updated for this session
          (bind _returnvalue (Class|VictoryCore|GetClassDefaultObject (Utilities|GetClass self)))
          (bind _asarkframe_buff_bp_c (Utilities|Casting|CastToArkFrame_Buff_BP _returnvalue)))))))

(fn ConstructionScript
  (|CallParentFunction))

(fn NotifyDamage
  (params (DamageAmount :type Float%20%28single-precision%29) (DamageClass :type Damage%20Type%20Class%20Reference) (EventInstigator :type Controller%20Object%20Reference) (TheDamageCauser :type Actor%20Object%20Reference))
  (|CallParentFunction DamageAmount DamageClass EventInstigator TheDamageCauser)
  (Class|ArkFrameLogicExpansionInterface|ExpandedNotifyDamage(Message) (Variables|ArkFrame|System|GetLogicExpansions) DamageAmount DamageClass EventInstigator TheDamageCauser))

(fn NotifyBumpedPawn
  (params (BumpedPawn :type Primal%20Character%20Object%20Reference))
  (|CallParentFunction BumpedPawn)
  (Class|ArkFrameLogicExpansionInterface|ExpandedNotifyBumpedPawn(Message) (Variables|ArkFrame|System|GetLogicExpansions) BumpedPawn))

(fn NotifyBumpedbyPawn
  (params (BumpedBy :type Primal%20Character%20Object%20Reference))
  (|CallParentFunction BumpedBy)
  (Default|ExpandedNotifyBumpedbyPawn (Variables|ArkFrame|System|GetLogicExpansions) BumpedBy))

(fn BuffTickServer
  (params (DeltaTime :type Float%20%28single-precision%29))
  (|CallParentFunction DeltaTime)
  (Class|ArkFrameLogicExpansionInterface|ExpandedBuffTickServer(Message) (Variables|ArkFrame|System|GetLogicExpansions) DeltaTime))

(fn BuffTickClient
  (params (DeltaTime :type Float%20%28single-precision%29))
  (|CallParentFunction DeltaTime)
  (Class|ArkFrameLogicExpansionInterface|ExpandedBuffTickClient(Message) (Variables|ArkFrame|System|GetLogicExpansions) DeltaTime))

(fn BPSetupforInstigator
  (params (ForInstigator :type Actor%20Object%20Reference))
  (|CallParentFunction ForInstigator)
  (Class|ArkFrameLogicExpansionInterface|ExpandedBPSetupforInstigator(Message) (Variables|ArkFrame|System|GetLogicExpansions) ForInstigator))

(fn BPResetBuffStart
  (|CallParentFunction)
  (Class|ArkFrameLogicExpansionInterface|ExpandedBPResetBuffStart(Message) (Variables|ArkFrame|System|GetLogicExpansions)))

(fn BPPreSetupforInstigator
  (params (ForInstigator :type Actor%20Object%20Reference))
  (|CallParentFunction ForInstigator)
  (Class|ArkFrameLogicExpansionInterface|ExpandedBPPreSetupforInstigator(Message) (Variables|ArkFrame|System|GetLogicExpansions) ForInstigator))

(fn BPInstigatorDied
  (|CallParentFunction)
  (Class|ArkFrameLogicExpansionInterface|ExpandedBPInstigatorDied(Message) (Variables|ArkFrame|System|GetLogicExpansions)))

(fn BPDrawBuffStatusHUD
  (params (HUD :type Shooter%20HUD%20Object%20Reference) (XPos :type Float%20%28single-precision%29) (YPos :type Float%20%28single-precision%29) (ScaleMult :type Float%20%28single-precision%29))
  (|CallParentFunction HUD XPos YPos ScaleMult)
  (Class|ArkFrameLogicExpansionInterface|ExpandedBPDrawBuffStatusHUD(Message) (Variables|ArkFrame|System|GetLogicExpansions) HUD XPos YPos ScaleMult))

(fn BPDeactivated
  (params (ForInstigator :type Actor%20Object%20Reference))
  (|CallParentFunction ForInstigator)
  (Class|ArkFrameLogicExpansionInterface|ExpandedBPDeactivated(Message) (Variables|ArkFrame|System|GetLogicExpansions) ForInstigator))

(fn BPActivated
  (params (ForInstigator :type Actor%20Object%20Reference))
  (|CallParentFunction ForInstigator)
  (Class|ArkFrameLogicExpansionInterface|ExpandedBPActivated(Message) (Variables|ArkFrame|System|GetLogicExpansions) ForInstigator))

(fn DrawBasicFloatingHUD
  (params (ForHUD :type HUD%20Object%20Reference))
  (|CallParentFunction ForHUD)
  (Class|ArkFrameLogicExpansionInterface|ExpandedDrawBasicFloatingHUD(Message) (Variables|ArkFrame|System|GetLogicExpansions) ForHUD))

(fn BPPreInitializeComponents
  (|CallParentFunction)
  (Class|ArkFrameLogicExpansionInterface|ExpandedBPPreInitializeComponents(Message) (Variables|ArkFrame|System|GetLogicExpansions)))

(fn BPPostInitializeComponents
  (|CallParentFunction)
  (Class|ArkFrameLogicExpansionInterface|ExpandedBPPostInitializeComponents(Message) (Variables|ArkFrame|System|GetLogicExpansions)))

(fn BPInventoryItemUsed
  (params (InventoryItemObject :type Object%20Object%20Reference))
  (|CallParentFunction InventoryItemObject)
  (Class|ArkFrameLogicExpansionInterface|ExpandedBPInventoryItemUsed(Message) (Variables|ArkFrame|System|GetLogicExpansions) InventoryItemObject))

(fn BPInventoryItemDropped
  (params (InventoryItemObject :type Object%20Object%20Reference))
  (|CallParentFunction InventoryItemObject)
  (Class|ArkFrameLogicExpansionInterface|ExpandedBPInventoryItemDropped(Message) (Variables|ArkFrame|System|GetLogicExpansions) InventoryItemObject))

(fn BPChangedActorTeam
  (|CallParentFunction)
  (Class|ArkFrameLogicExpansionInterface|ExpandedBPChangedActorTeam(Message) (Variables|ArkFrame|System|GetLogicExpansions)))

(fn BPAttachedRootComponent
  (|CallParentFunction)
  (Class|ArkFrameLogicExpansionInterface|ExpandedBPAttachedRootComponent(Message) (Variables|ArkFrame|System|GetLogicExpansions)))

(fn UpdateBuffPersistentData
  (|CallParentFunction)
  (Class|ArkFrameLogicExpansionInterface|ExpandedUpdateBuffPersistentData(Message) (Variables|ArkFrame|System|GetLogicExpansions)))

(fn SetBuffCauser
  (params (CausedBy :type Actor%20Object%20Reference))
  (|CallParentFunction CausedBy)
  (Class|ArkFrameLogicExpansionInterface|ExpandedSetBuffCauser(Message) (Variables|ArkFrame|System|GetLogicExpansions) CausedBy))

(fn DrawBuffFloatingHUD
  (params (BuffIndex :type Integer) (HUD :type Shooter%20HUD%20Object%20Reference) (CenterX :type Float%20%28single-precision%29) (CenterY :type Float%20%28single-precision%29) (DrawScale :type Float%20%28single-precision%29))
  (|CallParentFunction BuffIndex HUD CenterX CenterY DrawScale)
  (Class|ArkFrameLogicExpansionInterface|ExpandedDrawBuffFloatingHUD(Message) (Variables|ArkFrame|System|GetLogicExpansions) BuffIndex HUD CenterX CenterY DrawScale))

(fn RecieveMatineeUpdated
  (|CallParentFunction)
  (Class|ArkFrameLogicExpansionInterface|ExpandedRecieveMatineeUpdated(Message) (Variables|ArkFrame|System|GetLogicExpansions)))

(fn K2onEndViewTarget
  (params (PC :type Player%20Controller%20Object%20Reference))
  (|CallParentFunction PC)
  (Class|ArkFrameLogicExpansionInterface|ExpandedonEndViewTarget(Message) (Variables|ArkFrame|System|GetLogicExpansions) PC))

(fn K2onBecomeViewTarget
  (params (PC :type Player%20Controller%20Object%20Reference))
  (|CallParentFunction PC)
  (Class|ArkFrameLogicExpansionInterface|ExpandedonBecomeViewTarget(Message) (Variables|ArkFrame|System|GetLogicExpansions) PC))

(fn ReceiveRadialDamage
  (params (DamageReceived :type Float%20%28single-precision%29) (DamageType :type Damage%20Type%20Object%20Reference) (Origin :type Vector :default "0, 0, 0") (HitInfo :type Hit%20Result%20Structure%20%28by%20ref%29) (InstigatedBy :type Controller%20Object%20Reference) (DamageCauser :type Actor%20Object%20Reference))
  (|CallParentFunction DamageReceived DamageType Origin HitInfo InstigatedBy DamageCauser)
  (Class|ArkFrameLogicExpansionInterface|ExpandedRadialDamage(Message) (Variables|ArkFrame|System|GetLogicExpansions) DamageReceived DamageType Origin HitInfo InstigatedBy DamageCauser)
  (return))

(fn ReceivePointDamage
  (params (Damage :type Float%20%28single-precision%29) (DamageType :type Damage%20Type%20Object%20Reference) (HitLocation :type Vector :default "0, 0, 0") (HitNormal :type Vector :default "0, 0, 0") (HitComponent :type Primitive%20Component%20Object%20Reference) (BoneName :type Name :default "None") (ShotFromDirection :type Vector :default "0, 0, 0") (InstigatedBy :type Controller%20Object%20Reference) (DamageCauser :type Actor%20Object%20Reference))
  (|CallParentFunction Damage DamageType HitLocation HitNormal HitComponent BoneName ShotFromDirection InstigatedBy DamageCauser)
  (Class|ArkFrameLogicExpansionInterface|ExpandedPointDamage(Message) (Variables|ArkFrame|System|GetLogicExpansions) Damage DamageType HitLocation HitNormal HitComponent BoneName ShotFromDirection InstigatedBy DamageCauser))

(fn ReceiveAnyDamage
  (params (Damage :type Float%20%28single-precision%29) (DamageType :type Damage%20Type%20Object%20Reference) (InstigatedBy :type Controller%20Object%20Reference) (DamageCauser :type Actor%20Object%20Reference))
  (|CallParentFunction Damage DamageType InstigatedBy DamageCauser)
  (Class|ArkFrameLogicExpansionInterface|ExpandedAnyDamage(Message) (Variables|ArkFrame|System|GetLogicExpansions) Damage DamageType InstigatedBy DamageCauser))

(fn ReceiveHit
  (params (MyComp :type Primitive%20Component%20Object%20Reference) (Other :type Actor%20Object%20Reference) (OtherComp :type Primitive%20Component%20Object%20Reference) (bSelfMoved :type Boolean) (HitLocation :type Vector :default "0, 0, 0") (HitNormal :type Vector :default "0, 0, 0") (NormalImpulse :type Vector :default "0, 0, 0") (Hit :type Hit%20Result%20Structure%20%28by%20ref%29))
  (|CallParentFunction MyComp Other OtherComp bSelfMoved HitLocation HitNormal NormalImpulse Hit)
  (Class|ArkFrameLogicExpansionInterface|ExpandedHit(Message) (Variables|ArkFrame|System|GetLogicExpansions) MyComp Other OtherComp bSelfMoved HitLocation HitNormal NormalImpulse Hit)
  (return))

(fn ReceiveActorEndOverlap
  (params (OtherActor :type Actor%20Object%20Reference))
  (|CallParentFunction OtherActor)
  (Class|ArkFrameLogicExpansionInterface|ExpandedActorEndOverlap(Message) (Variables|ArkFrame|System|GetLogicExpansions) OtherActor))

(fn ReceiveActorBeginOverlap
  (params (OtherActor :type Actor%20Object%20Reference))
  (|CallParentFunction OtherActor)
  (Class|ArkFrameLogicExpansionInterface|ExpandedActorBeginOverlap(Message) (Variables|ArkFrame|System|GetLogicExpansions) OtherActor))