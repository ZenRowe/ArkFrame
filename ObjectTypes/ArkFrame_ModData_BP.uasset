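; ArkFrame mod data singleton actor that registers its mod information with the ArkFrame negotiator through the game mode.
; On the authority, a looping timer started shortly after BeginPlay retries registration in case the negotiator has not finished instantiating.
; Success clears the timer and sets a short lifespan so the actor destroys itself, while creation, attempts and failures go to a live event trace log.
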(event Custom|Timer_RegistrationTry
  ;[1 1 1] Attempt to register with the negotiater, and if successful destroy this actor
  (CallFunction|CreateLiveEventTraceLog self "A mod started making an attempt to resgister" "NewEnumerator0")
  (if true
    (bind _bisregistered (Class|ArkFrameManagerInterface|RegisterMod(Message) (Game|GetGameMode) (Variables|ArkFrame|GetModInformation)))
    (if _bisregistered
      (Utilities|Time|ClearTimerbyFunctionName 0 "Timer_RegistrationTry")
      (Actor|SetLifeSpan 5.0)
      (else
        (CallFunction|CreateLiveEventTraceLog self "Mod failed to register" "NewEnumerator2")))
    (else
      (CallFunction|CreateLiveEventTraceLog self "ArkFrame negotiator could not be found to register" "NewEnumerator2"))))

(event EventBeginPlay
  ;[1 1 1] Set a timer to retry registration in case the negotiator has not fully instantiated yet
  (Utilities|FlowControl|Delay 0.2)
  (Networking|SwitchHasAuthority
    (:Authority
      (Utilities|Time|SetTimerbyFunctionName 0 "Timer_RegistrationTry" 0.2 true)
      (CallFunction|CreateLiveEventTraceLog self "Arkframe mod data singleton created" "NewEnumerator0"))))

(fn ConstructionScript)