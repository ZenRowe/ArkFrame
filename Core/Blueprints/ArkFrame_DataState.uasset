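; ArkFrame_DataState is the ArkFrame modding framework's shared state actor, holding the mod registry, resource dictionary, mod configs and live event trace logs.
; On authority the first instance registers with the ArkFrame manager, retrying by timer, and others destroy themselves.
; Authority-guarded functions set state, save mod configs to save slots, and record capped, newest-first trace logs mirrored to the server log.
; Lookups resolve resources, class owners and global or per-mod tracing.
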(event Custom|Retry_OnInitDataState
  (bind _arkframemanager (CallFunction|GetArkFrameManager))
  (Utilities|IsValid _arkframemanager
    (:Is%20Valid
      (Utilities|Time|ClearTimerbyFunctionName self "Retry_OnInitDataState")
      (bind _asarkframe_manager_c (Utilities|Casting|CastToArkFrame_Manager _arkframemanager))
      (Default|OnInitArkFrameDataState _asarkframe_manager_c))))

(event EventBeginPlay
  (bind _arkframemanager (CallFunction|GetArkFrameManager))
  (Utilities|FlowControl|RetriggerableDelay 0.2)
  (Networking|SwitchHasAuthority
    (:Authority
      (bind _outactors (Actor|GetAllActorsOfClass "ArkFrame_DataState_C"))
      (if (== (Utilities|Array|Get(acopy) _outactors) self)
        (Utilities|IsValid _arkframemanager
          (:Is%20Valid
            (bind _asarkframe_manager_c (Utilities|Casting|CastToArkFrame_Manager _arkframemanager))
            (Default|OnInitArkFrameDataState _asarkframe_manager_c))
          (:Is%20Not%20Valid
            (Utilities|Time|SetTimerbyFunctionName self "Retry_OnInitDataState" 0.2 true)))
        (else
          (Actor|DestroyActor))))))

(fn ConstructionScript)

(fn SetArkFrameReady
  (Networking|SwitchHasAuthority
    (:Authority
      (Variables|ArkFrame|System|SetbIsArkFrameReady true true))))

(fn SetResourceDictionary
  (params (ResourceDictionary :type Array%20of%20F%20Ark%20Frame%20Resource%20Dictionary%20Item%20Structures))
  (Networking|SwitchHasAuthority
    (:Authority
      (Variables|ArkFrame|System|SetResourceDictionary ResourceDictionary true))))

(fn SetGlobalEventTracingState
  (params (bEventTracingState :type Boolean))
  (Networking|SwitchHasAuthority
    (:Authority
      (Variables|ArkFrame|EventTrace|SetbIsGlobalEventTracingEnabled bEventTracingState true))))

(fn SetEventTraceStateforMod
  (params (ForMod :type Name) (bNewState :type Boolean))
  (bind (_array_element _array_index) (Utilities|Array|ForEachLoopwithBreak (Variables|ArkFrame|System|GetModCollection) :!label _label)
    (:LoopBody
      (LocalVariables|SetL_ModInfo _array_element)
      (if (Utilities|Name|Equal(Name) (.ModName (Utilities|Struct|BreakFArkFrame_ModInfo _array_element)) ForMod)
        (Utilities|Struct|SetmembersinFArkFrame_ModInfo (LocalVariables|GetL_ModInfo) bNewState)
        (Utilities|Array|SetArrayElem (Variables|ArkFrame|System|GetModCollection) _array_index (LocalVariables|GetL_ModInfo))
        (goto _label Break)))
    (:Completed
      (Class|Actor|ForceReplicateNow false false))))

(fn OnRepLiveEventTraceLogs
  (Default|CallBPNotifyLiveEventTraceEntry (Utilities|Array|Get(acopy) (Variables|ArkFrame|EventTrace|GetLiveEventTraceLogs))))

(fn CheckArkFrameStatus
  (return (Variables|ArkFrame|System|GetbIsArkFrameReady)))

(fn FindSourceModbyObjectClass
  (params (ObjectClass :type Object%20Class%20Reference))
  ;[1 1 1] From each mod collection, check for which mod owns the class provided (If any)
  (bind _array_element (Utilities|Array|ForEachLoopwithBreak (Variables|ArkFrame|System|GetModCollection) :!label _label)
    (:LoopBody
      (for _array_element_2 (.ClassRegistry (Utilities|Struct|BreakFArkFrame_ModInfo _array_element))
        (if (== _array_element_2 ObjectClass)
          (LocalVariables|SetL_ModName (.ModName (Utilities|Struct|BreakFArkFrame_ModInfo _array_element)))
          (goto _label Break))))
    (:Completed
      (return (LocalVariables|GetL_ModName)))))

(fn GetBulkLiveEventTraceLogs
  (return (Variables|ArkFrame|EventTrace|GetLiveEventTraceLogs)))

(fn GetConfigDataforMod
  (params (ModName :type Name :default "None"))
  (Networking|SwitchHasAuthority
    (:Authority
      ;[1 1 1] Check for existing config data
      (bind _array_element (Utilities|Array|ForEachLoopwithBreak (Variables|ArkFrame|System|GetModConfigObjects) :!label _label)
        (:LoopBody
          (bind _sourcemod (CallFunction|FindSourceModbyObjectClass (Utilities|GetClass _array_element)))
          (if (Utilities|Name|Equal(Name) _sourcemod ModName)
            (LocalVariables|SetL_SaveGameObject _array_element)
            (CallFunction|CreateLiveEventTraceLog self (Utilities|String|Append "Mod config loaded from cache: " (Utilities|String|ToString(Name) ModName)) "NewEnumerator0")
            (goto _label Break)))
        (:Completed
          (return (LocalVariables|GetL_SaveGameObject)))))
    (:Remote
      (return (LocalVariables|GetL_SaveGameObject)))))

(fn GetLiveEventTraceMode
  (params (SourceMod :type Name :default "None"))
  ;[1 1 1] Check global setting first
  (if (Variables|ArkFrame|EventTrace|GetbIsGlobalEventTracingEnabled)
    (LocalVariables|SetbL_IsTracingEnabled true)
    (else
      ;[1 1 1] If global setting is false, check per mod setting
      (bind _array_element (Utilities|Array|ForEachLoopwithBreak (Variables|ArkFrame|System|GetModCollection) :!label _label)
        (:LoopBody
          (if (Utilities|Name|Equal(Name) SourceMod (.ModName (Utilities|Struct|BreakFArkFrame_ModInfo _array_element)))
            (LocalVariables|SetbL_IsTracingEnabled (.bIsLiveEventTracingEnabled (Utilities|Struct|BreakFArkFrame_ModInfo _array_element)))
            (goto _label Break)
            (else
              _)))
        (:Completed
          _))))
  (return (LocalVariables|GetbL_IsTracingEnabled)))

(fn GetModRegistry
  (return (Variables|ArkFrame|System|GetModCollection)))

(fn GetResourcebyKey
  (params (ResourceKey :type Name :default "None"))
  (bind _variable (|TemporaryVariable))
  (|Assign _variable (Class|KismetSystemLibrary|MakeLiteralBool false))
  (bind _array_element (Utilities|Array|ForEachLoopwithBreak (Variables|ArkFrame|System|GetResourceDictionary) :!label _label)
    (:LoopBody
      (if (Utilities|Name|Equal(Name) ResourceKey (.ResourceKey (Utilities|Struct|BreakFArkFrame_ResourceDictionaryItem _array_element)))
        (|Assign _variable (Utilities|Name|Equal(Name) ResourceKey (.ResourceKey (Utilities|Struct|BreakFArkFrame_ResourceDictionaryItem _array_element))))
        (LocalVariables|SetL_ResourceClass (.ResourceClassTemplate (Utilities|Struct|BreakFArkFrame_ResourceDictionaryItem _array_element)))
        (goto _label Break)))
    (:Completed
      (return _variable (LocalVariables|GetL_ResourceClass)))))

(fn SaveConfigDataforMod
  (params (ModName :type Name :default "None"))
  (Networking|SwitchHasAuthority
    (:Authority
      (bind _array_element (Utilities|Array|ForEachLoopwithBreak (Variables|ArkFrame|System|GetModCollection) :!label _label)
        (:LoopBody
          (if (Utilities|Name|Equal(Name) (.ModName (Utilities|Struct|BreakFArkFrame_ModInfo _array_element)) ModName)
            (for _array_element_2 (Variables|ArkFrame|System|GetModConfigObjects)
              (if (== (Utilities|GetClass _array_element_2) (.ConfigSaveClass (Utilities|Struct|BreakFArkFrame_ModInfo _array_element)))
                (bind _returnvalue (SaveGame|SaveGametoSlot _array_element_2 (Utilities|String|Append "ArkFrame/" (Utilities|String|ToString(Name) ModName))))
                (ArkFrame|EventTrace|SetEventTraceStateforMod ModName (Variables|/Game/Mods/ArkFrame/ObjectTypes/ModConfigs/ArkFrame_ModConfigSave.ArkFrame_ModConfigSave_C|GetbEnableModEventTracing _array_element_2))
                (if _returnvalue
                  (CallFunction|CreateLiveEventTraceLog self (Utilities|String|Append "Mod data saved: " (Utilities|String|ToString(Name) ModName)) "NewEnumerator0" _array_element_2)
                  (goto _label Break)
                  (else
                    (CallFunction|CreateLiveEventTraceLog self (Utilities|String|Append "Mod data failed to save: " (Utilities|String|ToString(Name) ModName)) "NewEnumerator2")
                    (goto _label Break)))))))
        (:Completed
          (return true))))
    (:Remote
      (return true))))

(fn SubmitEventTraceLog
  (params (LiveEventTraceEntry :type F%20Ark%20Frame%20Live%20Event%20Trace%20Entry%20Structure))
  (bind (_sourcemod _timestamp _priority _instance _sourceobject _relatedobject _entrystring) (Utilities|Struct|BreakFArkFrame_LiveEventTraceEntry LiveEventTraceEntry))
  (bind _liveeventtracelogs (Variables|ArkFrame|EventTrace|GetLiveEventTraceLogs))
  (Networking|SwitchHasAuthority
    (:Authority
      (Utilities|FlowControl|Sequence
        (:then_0
          (bind _asshootergamemode (Utilities|Casting|CastToShooterGameMode (Game|GetGameMode)))
          (Class|ShooterGameMode|PrinttoServerGameLog _asshootergamemode (Utilities|String|ToString(Text) (Utilities|Text|FormatText "{Mod} - {Instance}: {Entry}" (Utilities|Text|ToText(Name) _sourcemod) (Utilities|Text|ToText(String) _instance) (Utilities|Text|ToText(String) _entrystring))) false))
        (:then_1
          (Utilities|Array|Insert _liveeventtracelogs LiveEventTraceEntry)
          (if (> (Utilities|Array|Length _liveeventtracelogs) (Variables|ArkFrame|EventTrace|GetMaxEventLogSize))
            (Utilities|Array|RemoveIndex _liveeventtracelogs (Utilities|Array|LastIndex _liveeventtracelogs)))
          (return true))))))