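; ArkFrame's singleton manager actor, which negotiates between registered mods and the game.
; Mod registration and data-state init restart a retriggerable delay, batching one build of mod configs, a save-persisted resource dictionary and keybinds, then map actor replacement and the ready flag.
; Getters serve mods' harvest resources, inventory items and logic expansions matched by unique name or AND/OR/NAND/NOR tag rules.
; Harvest entries are also checked against the dictionary to drop replaceable duplicate resources.
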(event Custom|Delay_BuildDataSets
  (Utilities|FlowControl|RetriggerableDelay 5.0)
  (Utilities|FlowControl|Sequence
    (:then_0
      (ArkFrame|System|LoadModConfigs))
    (:then_1
      (ArkFrame|System|BuildResourceDictionary))
    (:then_2
      (ArkFrame|System|BuildKeybindDataSet))
    (:then_3
      (ArkFrame|System|DoReplaceMapActors))
    (:then_4
      (bind _asarkframe_datastate_c (Utilities|Casting|CastToArkFrame_DataState (CallFunction|GetArkFrameDataState)))
      (Default|SetArkFrameReady _asarkframe_datastate_c)
      (CallFunction|CreateLiveEventTraceLog self "ArkFrame Ready to accept incoming requests" "NewEnumerator0"))))

(event EventBeginPlay
  (Utilities|FlowControl|RetriggerableDelay 0.2)
  (bind _outactors (Actor|GetAllActorsOfClass "ArkFrame_Manager_C"))
  (if (== (Utilities|Array|Get(acopy) _outactors) self)
    (Variables|ArkFrame|System|SetArkFrameSessionID (Math|DateTime|Now))
    (else
      (Actor|DestroyActor))))

(fn ConstructionScript)

(fn BuildResourceDictionary
  (bind _asarkframe_datastate_c (Utilities|Casting|CastToArkFrame_DataState (CallFunction|GetArkFrameDataState)))
  (LocalVariables|SetL_DataState _asarkframe_datastate_c)
  (Utilities|FlowControl|Sequence
    (:then_0
      ;[1 1 1] Load resource dictionary state save object and remove any empties (Removed mods)
      (Default|SetResourceDictionary (LocalVariables|GetL_DataState) (Variables|/Game/Mods/ArkFrame/Core/Blueprints/ArkFrame_CoreSaveData.ArkFrame_CoreSaveData_C|GetResourceDictionaryState (Variables|ArkFrame|System|GetArkFrameCoreSaveData)))
      (bind (_array_element _array_index) (Utilities|Array|ForEachLoopwithBreak (Variables|/Game/Mods/ArkFrame/Core/Blueprints/ArkFrame_DataState.ArkFrame_DataState_C|GetResourceDictionary (LocalVariables|GetL_DataState)) :!label _label)
        (:LoopBody
          (if (== (.ResourceClassTemplate (Utilities|Struct|BreakFArkFrame_ResourceDictionaryItem _array_element)) 0)
            (Utilities|Array|RemoveIndex (Variables|/Game/Mods/ArkFrame/Core/Blueprints/ArkFrame_DataState.ArkFrame_DataState_C|GetResourceDictionary (LocalVariables|GetL_DataState)) _array_index)
            (Utilities|FlowControl|Sequence
              (:then_0
                (goto _label Break))
              (:then_1
                (goto _label)))))))
    (:then_1
      ;[1 1 1] Parse all registered mods for first unique resource key entry
      (for _array_element_2 (Variables|/Game/Mods/ArkFrame/Core/Blueprints/ArkFrame_DataState.ArkFrame_DataState_C|GetModCollection (LocalVariables|GetL_DataState))
        (for _array_element_3 (.ResourceClassDefinitions (Utilities|Struct|BreakFArkFrame_ModInfo _array_element_2))
          (LocalVariables|SetbL_MatchFound false)
          (for _array_element_4 (Variables|/Game/Mods/ArkFrame/Core/Blueprints/ArkFrame_DataState.ArkFrame_DataState_C|GetResourceDictionary (LocalVariables|GetL_DataState))
            (bind _returnvalue (Class|VictoryCore|GetClassDefaultObject _array_element_3))
            (bind _asarkframe_resource_bp_c (Utilities|Casting|CastToArkFrame_Resource_BP _returnvalue))
            (if (and (Utilities|Name|Equal(Name) (Variables|/Game/Mods/ArkFrame/ObjectTypes/Items/ArkFrame_Resource_BP.ArkFrame_Resource_BP_C|GetResourceKey _asarkframe_resource_bp_c) (.ResourceKey (Utilities|Struct|BreakFArkFrame_ResourceDictionaryItem _array_element_4))) (Utilities|ClassIsChildOf (.ResourceClassTemplate (Utilities|Struct|BreakFArkFrame_ResourceDictionaryItem _array_element_4)) "/Game/Mods/ArkFrame/ObjectTypes/Items/ArkFrame_Resource_BP.ArkFrame_Resource_BP_C"))
              (LocalVariables|SetbL_MatchFound true)))
          (if (not (LocalVariables|GetbL_MatchFound))
            (bind _returnvalue_2 (Class|VictoryCore|GetClassDefaultObject _array_element_3))
            (bind _asarkframe_resource_bp_c_2 (Utilities|Casting|CastToArkFrame_Resource_BP _returnvalue_2))
            (Utilities|Array|Add (Variables|/Game/Mods/ArkFrame/Core/Blueprints/ArkFrame_DataState.ArkFrame_DataState_C|GetResourceDictionary (LocalVariables|GetL_DataState)) (Utilities|Struct|MakeFArkFrame_ResourceDictionaryItem (Variables|/Game/Mods/ArkFrame/ObjectTypes/Items/ArkFrame_Resource_BP.ArkFrame_Resource_BP_C|GetResourceKey _asarkframe_resource_bp_c_2) _array_element_3))))))
    (:then_2
      ;[1 1 1] Save any resource dictionary changes to file
      (Variables|/Game/Mods/ArkFrame/Core/Blueprints/ArkFrame_CoreSaveData.ArkFrame_CoreSaveData_C|SetResourceDictionaryState (Variables|ArkFrame|System|GetArkFrameCoreSaveData) (Variables|/Game/Mods/ArkFrame/Core/Blueprints/ArkFrame_DataState.ArkFrame_DataState_C|GetResourceDictionary (LocalVariables|GetL_DataState)))
      (ArkFrame|System|SaveArkFrameData))
    (:then_3
      (CallFunction|CreateLiveEventTraceLog self (Utilities|String|Append "Resource dictionary built. Items: " (Utilities|String|ToString(Integer) (Utilities|Array|Length (Variables|/Game/Mods/ArkFrame/Core/Blueprints/ArkFrame_DataState.ArkFrame_DataState_C|GetResourceDictionary (LocalVariables|GetL_DataState))))) "NewEnumerator0"))
    (:then_4
      (return (Utilities|Array|Length (Variables|/Game/Mods/ArkFrame/Core/Blueprints/ArkFrame_DataState.ArkFrame_DataState_C|GetResourceDictionary (LocalVariables|GetL_DataState)))))))

(fn BuildKeybindDataSet
  (bind _keybinddataset (Variables|ArkFrame|System|GetKeybindDataSet))
  (bind _asarkframe_datastate_c (Utilities|Casting|CastToArkFrame_DataState (CallFunction|GetArkFrameDataState)))
  (for _array_element (Variables|/Game/Mods/ArkFrame/Core/Blueprints/ArkFrame_DataState.ArkFrame_DataState_C|GetModCollection _asarkframe_datastate_c)
    (Utilities|Array|AppendArray _keybinddataset (.KeybindDefinitions (Utilities|Struct|BreakFArkFrame_ModInfo _array_element)))
    (Utilities|FlowControl|Sequence
      (:then_0
        (CallFunction|CreateLiveEventTraceLog self (Utilities|String|Append "Keybind dataset constructed. Items: " (Utilities|String|ToString(Integer) (Utilities|Array|Length _keybinddataset))) "NewEnumerator0"))
      (:then_1
        (return (Utilities|Array|Length (Variables|ArkFrame|System|GetKeybindDataSet)))))))

(fn LoadArkFrameSave
  (bind _returnvalue (Class|VictoryCore|GetClassDefaultObject (Variables|ArkFrame|GetArkFrameCoreDataSaveClass)))
  (bind _asarkframe_coresavedata_c (Utilities|Casting|CastToArkFrame_CoreSaveData _returnvalue))
  (bind _returnvalue_2 (SaveGame|DoesSaveGameExist (Variables|/Game/Mods/ArkFrame/Core/Blueprints/ArkFrame_CoreSaveData.ArkFrame_CoreSaveData_C|GetSaveSlotName _asarkframe_coresavedata_c) (Variables|/Game/Mods/ArkFrame/Core/Blueprints/ArkFrame_CoreSaveData.ArkFrame_CoreSaveData_C|GetUserIndex _asarkframe_coresavedata_c)))
  (if _returnvalue_2
    (bind _returnvalue_3 (SaveGame|LoadGamefromSlot (Variables|/Game/Mods/ArkFrame/Core/Blueprints/ArkFrame_CoreSaveData.ArkFrame_CoreSaveData_C|GetSaveSlotName _asarkframe_coresavedata_c) (Variables|/Game/Mods/ArkFrame/Core/Blueprints/ArkFrame_CoreSaveData.ArkFrame_CoreSaveData_C|GetUserIndex _asarkframe_coresavedata_c)))
    (bind _asarkframe_coresavedata_c_2 (Utilities|Casting|CastToArkFrame_CoreSaveData _returnvalue_3)
      (:then
        (Variables|ArkFrame|System|SetArkFrameCoreSaveData _asarkframe_coresavedata_c_2))
      (:CastFailed
        (bind _returnvalue_4 (SaveGame|CreateSaveGameObject (Variables|ArkFrame|GetArkFrameCoreDataSaveClass) :!label _label))
        (bind _asarkframe_coresavedata_c_3 (Utilities|Casting|CastToArkFrame_CoreSaveData _returnvalue_4)
          (:then
            (Variables|ArkFrame|System|SetArkFrameCoreSaveData _asarkframe_coresavedata_c_3)
            (ArkFrame|System|SaveArkFrameData))
          (:CastFailed
            _))))
    (else
      (goto _label)))
  (Utilities|IsValid (Variables|ArkFrame|System|GetArkFrameCoreSaveData)
    (:Is%20Valid
      (if (Utilities|IsValid (Variables|ArkFrame|System|GetArkFrameCoreSaveData))
        (bind _asarkframe_datastate_c (Utilities|Casting|CastToArkFrame_DataState (CallFunction|GetArkFrameDataState)))
        (Default|SetGlobalEventTracingState _asarkframe_datastate_c (Variables|/Game/Mods/ArkFrame/Core/Blueprints/ArkFrame_CoreSaveData.ArkFrame_CoreSaveData_C|GetbIsGlobalEventTracingEnabled (Variables|ArkFrame|System|GetArkFrameCoreSaveData)))
        (Utilities|FlowControl|Sequence
          (:then_0
            (CallFunction|CreateLiveEventTraceLog self "ArkFrame save data loaded" "NewEnumerator0" (Variables|ArkFrame|System|GetArkFrameCoreSaveData)))
          (:then_1
            (return (Utilities|IsValid (Variables|ArkFrame|System|GetArkFrameCoreSaveData)))))
        (else
          (bind _asarkframe_datastate_c_2 (Utilities|Casting|CastToArkFrame_DataState (CallFunction|GetArkFrameDataState) :!label _label_2))
          (Default|SetGlobalEventTracingState _asarkframe_datastate_c_2 true)
          (Utilities|FlowControl|Sequence
            (:then_0
              (CallFunction|CreateLiveEventTraceLog self "ArkFrame save data failed to load Properly (Event tracing turned on as it's state could not be verified from save data)" "NewEnumerator2"))
            (:then_1
              (return (Utilities|IsValid (Variables|ArkFrame|System|GetArkFrameCoreSaveData))))))))
    (:Is%20Not%20Valid
      (goto _label_2))))

(fn SaveArkFrameData
  (bind _arkframecoresavedata (Variables|ArkFrame|System|GetArkFrameCoreSaveData))
  (Utilities|IsValid _arkframecoresavedata
    (:Is%20Valid
      (bind _returnvalue (SaveGame|SaveGametoSlot _arkframecoresavedata (Variables|/Game/Mods/ArkFrame/Core/Blueprints/ArkFrame_CoreSaveData.ArkFrame_CoreSaveData_C|GetSaveSlotName _arkframecoresavedata) (Variables|/Game/Mods/ArkFrame/Core/Blueprints/ArkFrame_CoreSaveData.ArkFrame_CoreSaveData_C|GetUserIndex _arkframecoresavedata)))
      (if _returnvalue
        (CallFunction|CreateLiveEventTraceLog self "Manager saved ArkFrame data" "NewEnumerator0" (Variables|ArkFrame|System|GetArkFrameCoreSaveData))
        (else
          (CallFunction|CreateLiveEventTraceLog self "ArkFrame data failed to save!" "NewEnumerator2" :!label _label))))
    (:Is%20Not%20Valid
      (goto _label))))

(fn MatchDescriptiveTags
  (params (DescriptiveTags :type Array%20of%20Names) (MatchingRules :type Array%20of%20F%20Ark%20Frame%20Sub%20Tag%20Query%20Group%20Structures))
  (bind _variable (|TemporaryVariable))
  (bind _variable_2 (|TemporaryVariable))
  (bind _variable_3 (|TemporaryVariable))
  (bind _variable_4 (|TemporaryVariable))
  ;[1 1 1] Check match by descriptive tags
  (LocalVariables|SetbL_IsMatch true)
  (bind _array_element (Utilities|Array|ForEachLoopwithBreak MatchingRules :!label _label)
    (:LoopBody
      (switch Utilities|FlowControl|Switch|SwitchonEArkFrame_MatchLogicEnums (.MatchRule (Utilities|Struct|BreakFArkFrame_SubTagQueryGroup _array_element))
        (:NewEnumerator1
          ;[1 1 1] AND Matching
          (for _array_element_2 (.DescriptiveTags (Utilities|Struct|BreakFArkFrame_SubTagQueryGroup _array_element))
            (|Assign _variable (Class|KismetSystemLibrary|MakeLiteralBool false))
            (bind _array_element_3 (Utilities|Array|ForEachLoopwithBreak DescriptiveTags :!label _label_2)
              (:LoopBody
                (if (Utilities|Name|Equal(Name) _array_element_3 _array_element_2)
                  (|Assign _variable (Utilities|Name|Equal(Name) _array_element_3 _array_element_2))
                  (goto _label_2 Break)))
              (:Completed
                (if (not _variable)
                  (LocalVariables|SetbL_IsMatch false)
                  (goto _label Break))))))
        (:NewEnumerator2
          ;[1 1 1] OR matching
          (bind _array_element_4 (Utilities|Array|ForEachLoopwithBreak (.DescriptiveTags (Utilities|Struct|BreakFArkFrame_SubTagQueryGroup _array_element)) :!label _label_3)
            (:LoopBody
              (|Assign _variable_2 (Class|KismetSystemLibrary|MakeLiteralBool false))
              (for _array_element_5 DescriptiveTags
                (if (Utilities|Name|Equal(Name) _array_element_5 _array_element_4)
                  (|Assign _variable_2 (Utilities|Name|Equal(Name) _array_element_5 _array_element_4))
                  (goto _label_3 Break))))
            (:Completed
              (if (not _variable_2)
                (LocalVariables|SetbL_IsMatch false)
                (goto _label Break)))))
        (:NewEnumerator3
          ;[1 1 1] NAND matching
          (for _array_element_6 (.DescriptiveTags (Utilities|Struct|BreakFArkFrame_SubTagQueryGroup _array_element))
            (|Assign _variable_3 (Class|KismetSystemLibrary|MakeLiteralBool false))
            (bind _array_element_7 (Utilities|Array|ForEachLoopwithBreak DescriptiveTags :!label _label_4)
              (:LoopBody
                (if (Utilities|Name|Equal(Name) _array_element_7 _array_element_6)
                  (|Assign _variable_3 (Utilities|Name|Equal(Name) _array_element_7 _array_element_6))
                  (goto _label_4 Break)))
              (:Completed
                (if _variable_3
                  (LocalVariables|SetbL_IsMatch false)
                  (goto _label Break))))))
        (:NewEnumerator6
          ;[1 1 1] NOR matching
          (bind _array_element_8 (Utilities|Array|ForEachLoopwithBreak (.DescriptiveTags (Utilities|Struct|BreakFArkFrame_SubTagQueryGroup _array_element)) :!label _label_5)
            (:LoopBody
              (|Assign _variable_4 (Class|KismetSystemLibrary|MakeLiteralBool false))
              (for _array_element_9 DescriptiveTags
                (if (Utilities|Name|Equal(Name) _array_element_9 _array_element_8)
                  (|Assign _variable_4 (Utilities|Name|Equal(Name) _array_element_9 _array_element_8))
                  (goto _label_5 Break))))
            (:Completed
              (if _variable_4
                (LocalVariables|SetbL_IsMatch false)
                (goto _label Break)))))))
    (:Completed
      (return (LocalVariables|GetbL_IsMatch)))))

(fn LoadModConfigs
  (bind _asarkframe_datastate_c (Utilities|Casting|CastToArkFrame_DataState (CallFunction|GetArkFrameDataState)))
  (for _array_element (Variables|/Game/Mods/ArkFrame/Core/Blueprints/ArkFrame_DataState.ArkFrame_DataState_C|GetModCollection _asarkframe_datastate_c)
    ;[1 1 1] Load config data and if it doesn't exist, create it
    (bind _returnvalue (SaveGame|DoesSaveGameExist (Utilities|String|Append "ArkFrame/" (Utilities|String|ToString(Name) (.ModName (Utilities|Struct|BreakFArkFrame_ModInfo _array_element))))))
    (if _returnvalue
      (bind _returnvalue_2 (SaveGame|LoadGamefromSlot (Utilities|String|Append "ArkFrame/" (Utilities|String|ToString(Name) (.ModName (Utilities|Struct|BreakFArkFrame_ModInfo _array_element))))))
      (bind _asarkframe_modconfigsave_c (Utilities|Casting|CastToArkFrame_ModConfigSave _returnvalue_2)
        (:then
          (LocalVariables|SetL_SaveGameObject _asarkframe_modconfigsave_c)
          (Default|SetEventTraceStateforMod _asarkframe_datastate_c (.ModName (Utilities|Struct|BreakFArkFrame_ModInfo _array_element)) (Variables|/Game/Mods/ArkFrame/ObjectTypes/ModConfigs/ArkFrame_ModConfigSave.ArkFrame_ModConfigSave_C|GetbEnableModEventTracing _asarkframe_modconfigsave_c))
          (Utilities|Array|Add (Variables|/Game/Mods/ArkFrame/Core/Blueprints/ArkFrame_DataState.ArkFrame_DataState_C|GetModConfigObjects _asarkframe_datastate_c) (LocalVariables|GetL_SaveGameObject) :!label _label)
          (bind _returnvalue_3 (SaveGame|SaveGametoSlot (LocalVariables|GetL_SaveGameObject) (Utilities|String|Append "ArkFrame/" (Utilities|String|ToString(Name) (.ModName (Utilities|Struct|BreakFArkFrame_ModInfo _array_element))))))
          (if _returnvalue_3
            (CallFunction|CreateLiveEventTraceLog self (Utilities|String|Append "Mod Config Object created and saved successfully: " (Utilities|String|ToString(Name) (.ModName (Utilities|Struct|BreakFArkFrame_ModInfo _array_element)))) "NewEnumerator0" (LocalVariables|GetL_SaveGameObject))
            (else
              (CallFunction|CreateLiveEventTraceLog self (Utilities|String|Append "Mod Config Object failed to save:  " (Utilities|String|ToString(Name) (.ModName (Utilities|Struct|BreakFArkFrame_ModInfo _array_element)))) "NewEnumerator2"))))
        (:CastFailed
          (CallFunction|CreateLiveEventTraceLog self (Utilities|String|Append "Mod config save failed to load:" (Utilities|String|ToString(Name) (.ModName (Utilities|Struct|BreakFArkFrame_ModInfo _array_element)))) "NewEnumerator2")))
      (else
        (if (== (.ConfigSaveClass (Utilities|Struct|BreakFArkFrame_ModInfo _array_element)) 0)
          (bind _returnvalue_4 (SaveGame|CreateSaveGameObject "/Game/Mods/ArkFrame/ObjectTypes/ModConfigs/ArkFrame_ModConfigSave.ArkFrame_ModConfigSave_C"))
          (bind _asarkframe_modconfigsave_c_2 (Utilities|Casting|CastToArkFrame_ModConfigSave _returnvalue_4)
            (:then
              (LocalVariables|SetL_SaveGameObject _asarkframe_modconfigsave_c_2)
              (goto _label))
            (:CastFailed
              _))
          (else
            (bind _returnvalue_5 (SaveGame|CreateSaveGameObject (.ConfigSaveClass (Utilities|Struct|BreakFArkFrame_ModInfo _array_element))))
            (bind _asarkframe_modconfigsave_c_3 (Utilities|Casting|CastToArkFrame_ModConfigSave _returnvalue_5)
              (:then
                (LocalVariables|SetL_SaveGameObject _asarkframe_modconfigsave_c_3)
                (goto _label))
              (:CastFailed
                _))))
        (CallFunction|CreateLiveEventTraceLog self (Utilities|String|Append "Mod config save could not be created:" (Utilities|String|ToString(Name) (.ModName (Utilities|Struct|BreakFArkFrame_ModInfo _array_element)))) "NewEnumerator2"))))
  (return (Utilities|Array|Length (Variables|/Game/Mods/ArkFrame/Core/Blueprints/ArkFrame_DataState.ArkFrame_DataState_C|GetModConfigObjects _asarkframe_datastate_c))))

(fn DoReplaceMapActors
  (for _array_element (Variables|ArkFrame|GetMapActorsToReplace)
    (bind _asactor (Utilities|Casting|CastToActorClass (.FromClass (Utilities|Struct|BreakClassRemapping _array_element))))
    (bind _outactors (Actor|GetAllActorsOfClass _asactor))
    (bind _array_element_2 (Utilities|Array|ForEachLoopwithBreak _outactors :!label _label)
      (:LoopBody
        (bind _asactor_2 (Utilities|Casting|CastToActorClass (.ToClass (Utilities|Struct|BreakClassRemapping _array_element)))
          (:then
            (bind _returnvalue (Game|SpawnActorfromClass _asactor_2 (Transformation|GetActorTransform _array_element_2) true))
            (Actor|DestroyActor _array_element_2)
            (Class|Actor|ForceReplicateNow _array_element_2 false false))
          (:CastFailed
            (goto _label Break)))))))

(fn OnInitArkFrameDataState
  (Utilities|FlowControl|Sequence
    (:then_0
      (ArkFrame|System|LoadArkFrameSave))
    (:then_1
      (CallFunction|DelayBuildDataSets))))

(fn GetAdditionalHarvestableResources
  (params (HarvestComponentUniqueName :type Name :default "None") (DescriptiveTags :type Array%20of%20Names) (HarvestComponentClass :type Object%20Class%20Reference))
  (bind _asarkframe_datastate_c (Utilities|Casting|CastToArkFrame_DataState (CallFunction|GetArkFrameDataState)))
  (LocalVariables|SetL_DataState _asarkframe_datastate_c)
  (Utilities|FlowControl|Sequence
    (:then_0
      ;[0.14 0.008393 0.009729] Seed the buffer. This should be reworked to account for previous sessions somehow
      (bind _returnvalue (Class|VictoryCore|GetClassDefaultObject HarvestComponentClass))
      (bind _asprimalharvestingcomponent (Utilities|Casting|CastToPrimalHarvestingComponent _returnvalue))
      (LocalVariables|SetL_ResourceDefinitionBuffer (Variables|/Script/ShooterGame.PrimalHarvestingComponent|GetHarvestResourceEntries _asprimalharvestingcomponent)))
    (:then_1
      ;[1 1 1] Find Matching harvest entries
      (for _array_element (Variables|/Game/Mods/ArkFrame/Core/Blueprints/ArkFrame_DataState.ArkFrame_DataState_C|GetModCollection (LocalVariables|GetL_DataState))
        (for _array_element_2 (.AdditionalHarvestResources (Utilities|Struct|BreakFArkFrame_ModInfo _array_element))
          ;;[1 1 1] Match by unique name
          (if (.bShouldMatchByUniqueName (Utilities|Struct|BreakFArkFrame_AdditionalHarvestResources _array_element_2))
            (if (Utilities|Array|ContainsItem (.HarvestComponentUniqueNames (Utilities|Struct|BreakFArkFrame_AdditionalHarvestResources _array_element_2)) HarvestComponentUniqueName)
              (Utilities|Array|AppendArray (LocalVariables|GetL_ResourceDefinitionBuffer) (.HarvestResourceEntries (Utilities|Struct|BreakFArkFrame_AdditionalHarvestResources _array_element_2))))))
        ;;[1 1 1] Match by descriptive tags
        (bind _bismatch (ArkFrame|System|MatchDescriptiveTags DescriptiveTags (.DescriptiveTagsToMatch (Utilities|Struct|BreakFArkFrame_AdditionalHarvestResources _array_element_2))))
        (if _bismatch
          (Utilities|Array|AppendArray (LocalVariables|GetL_ResourceDefinitionBuffer) (.HarvestResourceEntries (Utilities|Struct|BreakFArkFrame_AdditionalHarvestResources _array_element_2))))))
    (:then_2
      ;[1 1 1] Validate entries against the resource dictionary
      (for _array_element_3 (LocalVariables|GetL_ResourceDefinitionBuffer)
        (bind _returnvalue_2 (Class|VictoryCore|GetClassDefaultObject (.ResourceItem (Utilities|Struct|BreakHarvestResourceEntry _array_element_3))))
        (bind _asarkframe_resource_bp_c (Utilities|Casting|CastToArkFrame_Resource_BP _returnvalue_2))
        (if (CallFunction|CheckAllowItemReplacement _asarkframe_resource_bp_c)
          (bind _array_element_4 (Utilities|Array|ForEachLoopwithBreak (Variables|/Game/Mods/ArkFrame/Core/Blueprints/ArkFrame_DataState.ArkFrame_DataState_C|GetResourceDictionary (LocalVariables|GetL_DataState)) :!label _label)
            (:LoopBody
              (if (Utilities|Name|Equal(Name) (Variables|/Game/Mods/ArkFrame/ObjectTypes/Items/ArkFrame_Resource_BP.ArkFrame_Resource_BP_C|GetResourceKey _asarkframe_resource_bp_c) (.ResourceKey (Utilities|Struct|BreakFArkFrame_ResourceDictionaryItem _array_element_4)))
                (if (== (.ResourceClassTemplate (Utilities|Struct|BreakFArkFrame_ResourceDictionaryItem _array_element_4)) (.ResourceItem (Utilities|Struct|BreakHarvestResourceEntry _array_element_3)))
                  (goto _label Break)
                  (else
                    (Utilities|Array|Add (LocalVariables|GetL_ResourceRemovalBuffer) _array_element_3)
                    (goto _label Break)))))))))
    (:then_3
      ;[1 1 1] Clear buffer
      (for _array_element_5 (LocalVariables|GetL_ResourceRemovalBuffer)
        (Utilities|Array|RemoveItem (LocalVariables|GetL_ResourceDefinitionBuffer) _array_element_5)))
    (:then_4
      ;[1 1 1] Return Entries
      (return (LocalVariables|GetL_ResourceDefinitionBuffer)))))

(fn GetAdditionalInventoryItems
  (params (InventoryUniqueName :type Name :default "None") (InventorySubTags :type Array%20of%20Names))
  (Utilities|FlowControl|Sequence
    (:then_0
      ;[1 1 1] Event Trace Log
      (CallFunction|CreateLiveEventTraceLog self (Utilities|String|Append "Additional Inventory items requested for inventory type: " (Utilities|String|ToString(Name) InventoryUniqueName)) "NewEnumerator0"))
    (:then_1
      (bind _asarkframe_datastate_c (Utilities|Casting|CastToArkFrame_DataState (CallFunction|GetArkFrameDataState)))
      (for _array_element (Variables|/Game/Mods/ArkFrame/Core/Blueprints/ArkFrame_DataState.ArkFrame_DataState_C|GetModCollection _asarkframe_datastate_c)
        (for _array_element_2 (.AddItemToInventory (Utilities|Struct|BreakFArkFrame_ModInfo _array_element))
          ;[1 1 1] Check match by unique name
          (if (.bShouldMatchByUniqueName (Utilities|Struct|BreakFArkFrame_InventoryAdditions _array_element_2))
            (if (Utilities|Array|ContainsItem (.InventoryUniqueNames (Utilities|Struct|BreakFArkFrame_InventoryAdditions _array_element_2)) InventoryUniqueName)
              (Utilities|Array|Add (LocalVariables|GetL_ReturnStructBuffer) _array_element_2))
            (else
              ;[1 1 1] Check match by descriptive tags
              (bind _bismatch (ArkFrame|System|MatchDescriptiveTags InventorySubTags (.DescriptiveTagsToMatch (Utilities|Struct|BreakFArkFrame_InventoryAdditions _array_element_2))))
              (if _bismatch
                (Utilities|Array|Add (LocalVariables|GetL_ReturnStructBuffer) _array_element_2))))))
      (return (LocalVariables|GetL_ReturnStructBuffer)))))

(fn GetArkFrameSessionID
  (return (Variables|ArkFrame|System|GetArkFrameSessionID)))

(fn GetKeybindClasses
  (return (Variables|ArkFrame|System|GetKeybindDataSet)))

(fn GetLogicExpansions
  (params (ActorUniqueName :type Name :default "None") (DescriptiveTags :type Array%20of%20Names))
  (Utilities|FlowControl|Sequence
    (:then_0
      ;[1 1 1] Event Trace Log
      (CallFunction|CreateLiveEventTraceLog self (Utilities|String|Append "Logic expansion templates requested: " (Utilities|String|ToString(Name) ActorUniqueName)) "NewEnumerator0"))
    (:then_1
      (bind _asarkframe_datastate_c (Utilities|Casting|CastToArkFrame_DataState (CallFunction|GetArkFrameDataState)))
      (for _array_element (Variables|/Game/Mods/ArkFrame/Core/Blueprints/ArkFrame_DataState.ArkFrame_DataState_C|GetModCollection _asarkframe_datastate_c)
        (for _array_element_2 (.LogicExpansions (Utilities|Struct|BreakFArkFrame_ModInfo _array_element))
          ;[1 1 1] Match by Unique Name
          (if (.bShouldMatchByUniqueName (Utilities|Struct|BreakFArkFrame_LogicExpansions _array_element_2))
            (if (Utilities|Array|ContainsItem (.ObjectUniqueNames (Utilities|Struct|BreakFArkFrame_LogicExpansions _array_element_2)) ActorUniqueName)
              (Utilities|Array|Add (LocalVariables|GetL_TemplateBuffer) (.LogicExpansionTemplate (Utilities|Struct|BreakFArkFrame_LogicExpansions _array_element_2))))
            (else
              ;[1 1 1] Match by Descriptive Tags
              (bind _bismatch (ArkFrame|System|MatchDescriptiveTags DescriptiveTags (.DescriptiveTagsToMatch (Utilities|Struct|BreakFArkFrame_LogicExpansions _array_element_2))))
              (if _bismatch
                (Utilities|Array|Add (LocalVariables|GetL_TemplateBuffer) (.LogicExpansionTemplate (Utilities|Struct|BreakFArkFrame_LogicExpansions _array_element_2))))))))
      (return (LocalVariables|GetL_TemplateBuffer)))))

(fn RegisterMod
  (params (ModInformation :type F%20Ark%20Frame%20Mod%20Info%20Structure))
  (bind _asarkframe_datastate_c (Utilities|Casting|CastToArkFrame_DataState (CallFunction|GetArkFrameDataState)))
  (Utilities|Array|Add (Variables|/Game/Mods/ArkFrame/Core/Blueprints/ArkFrame_DataState.ArkFrame_DataState_C|GetModCollection _asarkframe_datastate_c) ModInformation)
  (Utilities|FlowControl|Sequence
    (:then_0
      ;[1 1 1] Event Trace Log
      (CallFunction|CreateLiveEventTraceLog self (Utilities|String|Append "New mod registered with the negotiator: " (Utilities|String|ToString(Name) (.ModName (Utilities|Struct|BreakFArkFrame_ModInfo ModInformation)))) "NewEnumerator0"))
    (:then_1
      (CallFunction|DelayBuildDataSets))
    (:then_2
      (return true))))